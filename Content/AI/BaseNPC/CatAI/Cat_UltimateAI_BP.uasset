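; Cat AI NPC character with health, stance-based stagger and a limited lifetime that ends in placeholder self-detonation (print, then destroy).
; Hits launch it until depleted health or stance triggers ragdoll with pelvis knockback and disabled collision.
; Tick holds IsRagdolled-gated capsule-follow and timed pose-snapshot get-up logic, though that flag is never set true here.
; Physical animation drives bones below the spine outside ragdoll.
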(event `self.ReceiveBeginPlay`
  ;[1 1 1] Init variables
  (set `self.CurrentHealth` (`self._MaxHealth_`))
  (set `self.CurrentStance` (`self._MaxStance_`))
  (set `self.LifeTimer` (`self._LifeDuration_`))
  ;[1 1 1] Physical animation start
  (`PhysicalAnimationComponent.SetSkeletalMeshComponent` (`self.PhysicalAnimation`) (`self.Mesh`))
  (set `self.PhysicalAnimationSettings` (make `PhysicalAnimationData` true 1000.0 100.0 1000.0 100.0))
  (`self.PhysicalAnimTrigger` true))

(event `SelfDetonateAttack`
  ;[1 1 1] Death attack
  (`KismetSystemLibrary.PrintString` "EXPLOSION")
  (`KismetSystemLibrary.Delay` 0.5)
  (`self.K2_DestroyActor`))

(event `Health_TakeDamage`
  (params (Damage :type "Float (double-precision)"))
  ;[1 1 1] Health damage
  (bind _output_get (set `self.CurrentHealth` (- (`self.CurrentHealth`) Damage)))
  (if (<= _output_get 0.0)
    (set `self.IsDead` true)
    ;[1 1 1] Ragdoll physics and references
    (`PrimitiveComponent.SetSimulatePhysics` (`self.Mesh`) true :!label _label)
    (set `self.IsRagdolled` false)
    ;[1 1 1] Ragdoll Knockback
    (`PrimitiveComponent.AddImpulse` (`self.Mesh`) (* (* (`KismetMathLibrary.GetDirectionUnitVector` (stale `StaggerHit` AttackerVector) (`SceneComponent.K2_GetComponentLocation` (`self.CapsuleComponent`))) (* (stale `StaggerHit` StaggerMultiplier) 1000.0)) 1.0) "pelvis" true)
    (`/Game/UE4_Mannequin/Animations/ThirdPerson_AnimBP.FakeDeadYes` (cast `/Game/UE4_Mannequin/Animations/ThirdPerson_AnimBP` (`SkeletalMeshComponent.GetAnimInstance` (`self.Mesh`)) :!pure true))
    ;[1 1 1] Enable/Disable Hitboxes
    (set `PrimitiveComponent.bGenerateOverlapEvents` false (`self.HitBox`))
    (`PrimitiveComponent.SetCollisionProfileName` (`self.CapsuleComponent`) "NoCollision" true)))

(event `StaggerHit`
  (params (StaggerPower :type "Float (double-precision)") (AttackerVector :type "Vector Structure") (StaggerMultiplier :type "Float (double-precision)" :default 1.0))
  ;[1 1 1] Taking stagger damage
  (bind _output_get (set `self.CurrentStance` (- (`self.CurrentStance`) StaggerPower)))
  (if (<= _output_get 0.0)
    ;[1 1 1] Downed timer + get up
    (set `self.DownedTimer` (`self._DownedDuration_`))
    (goto _label)
    (else
      (`self.LaunchCharacter` (* (`KismetMathLibrary.GetDirectionUnitVector` AttackerVector (`SceneComponent.K2_GetComponentLocation` (`self.CapsuleComponent`))) (* StaggerMultiplier 1000.0)) true true))))

(event `CachePose`
  ;[1 1 1] Ragdoll physics and references
  ;;[1 1 1] Caching pose for animation
  (`KismetSystemLibrary.Delay` 0.0)
  (`KismetSystemLibrary.Delay` 0.0)
  (`AnimInstance.SavePoseSnapshot` (`SkeletalMeshComponent.GetAnimInstance` (`self.Mesh`)) "RagdollEnd"))

(event `self.ReceiveTick`
  (params (DeltaSeconds :type "Float (single-precision)"))
  (`|ExecutionSequence`
    (:`then_0`
      ;[1 1 1] Downed timer + get up
      (if (and (`self.IsRagdolled`) (not (`self.IsDead`)))
        (bind _output_get (set `self.DownedTimer` (- (`self.DownedTimer`) (`GameplayStatics.GetWorldDeltaSeconds`))))
        (if (<= _output_get 0.0)
          (set `self.CurrentStance` (`self._MaxStance_`))
          ;[1 1 1] Ragdoll physics and references
          (`self.CachePose`)
          (`KismetSystemLibrary.Delay` 0.1)
          (`PrimitiveComponent.SetSimulatePhysics` (`self.Mesh`) false)
          (set `self.IsRagdolled` false)
          (`/Game/UE4_Mannequin/Animations/ThirdPerson_AnimBP.FakeDeadNo` (cast `/Game/UE4_Mannequin/Animations/ThirdPerson_AnimBP` (`SkeletalMeshComponent.GetAnimInstance` (`self.Mesh`)) :!pure true))
          ;[1 1 1] Enable/Disable Hitboxes
          (set `PrimitiveComponent.bGenerateOverlapEvents` true (`self.HitBox`))
          (`PrimitiveComponent.SetCollisionProfileName` (`self.CapsuleComponent`) "Pawn" true)
          (`self.PhysicalAnimTrigger` true))))
    (:`then_1`
      ;[1 1 1] Capsule (root) follows when ragdolling
      (if (`self.IsRagdolled`)
        (`self.CalculateMeshLocation`)
        (`SceneComponent.K2_SetWorldLocation` (`self.CapsuleComponent`) (+ (`self.MeshLocation`) (0.0 0.0 64.0)) false false)
        (else
          (set `self.MeshLocation` (`SceneComponent.GetSocketLocation` (`self.Mesh`) "pelvis")))))
    (:`then_2`
      ;[1 1 1] Life countdown
      (bind _output_get_2 (set `self.LifeTimer` (- (`self.LifeTimer`) (`GameplayStatics.GetWorldDeltaSeconds`))))
      ;[1 1 1] Force Death
      (if (<= _output_get_2 0.0)
        (`/Engine/EditorBlueprintResources/StandardMacros.DoOnce` false
          (:`Completed`
            (`self.SelfDetonateAttack`)))))))

(fn `CalculateMeshLocation`
  (bind _returnvalue (`SceneComponent.GetSocketLocation` (`self.Mesh`) "pelvis"))
  (bind (_outhit _returnvalue_2) (`KismetSystemLibrary.LineTraceSingle` _returnvalue (+ _returnvalue (* (0.0 0.0 -1.0) 100.0)) "TraceTypeQuery1"))
  (if _returnvalue_2
    (set `self.BaseLocation` (`.Location` (`GameplayStatics.BreakHitResult` _outhit)))
    (else
      (set `self.BaseLocation` (`SceneComponent.GetSocketLocation` (`self.Mesh`) "pelvis"))))
  (set `self.MeshLocation` (+ (`KismetMathLibrary.VInterpTo` (`self.MeshLocation`) (`self.BaseLocation`) (`GameplayStatics.GetWorldDeltaSeconds`) 5.0) (0.0 0.0 0.05))))

(fn `PhysicalAnimTrigger`
  (params (Simulate :type Boolean))
  (bind _spine_01bone (`self.spine_01Bone`))
  (`PhysicalAnimationComponent.ApplyPhysicalAnimationSettingsBelow` (`self.PhysicalAnimation`) _spine_01bone (`self.PhysicalAnimationSettings`) true)
  (`SkeletalMeshComponent.SetAllBodiesBelowSimulatePhysics` (`self.Mesh`) _spine_01bone Simulate false))

(fn `UserConstructionScript`)