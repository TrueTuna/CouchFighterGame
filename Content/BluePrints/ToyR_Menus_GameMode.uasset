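; Menu game mode that runs main menu and local four-player character select, creating players at BeginPlay.
; Menu input events switch on GameArea to drive the linked UI, with wrapping selection indices and per-controller arrays for hover, join and ready state.
; Joining swaps a player's pawn for the hovered character with input disabled; leaving restores a spectator pawn.
; All-ready opens BaseLevel, and EndPlay from character select saves selections to the game instance.
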(event `self.ReceiveBeginPlay`
  (`|ExecutionSequence`
    (:`then_0`
      ;[1 1 1] Create 4 players
      (`GameplayStatics.CreatePlayer` 1)
      (`GameplayStatics.CreatePlayer` 2)
      (`GameplayStatics.CreatePlayer` 3))
    (:`then_1`
      ;[1 1 1] Set the level we are on
      (bind _returnvalue (`GameplayStatics.GetCurrentLevelName` true))
      (set `self._GameArea_` _returnvalue))
    (:`then_2`
      ;[1 1 1] Getting Character spawn points (keep for character select)
      (bind _outactors (`GameplayStatics.GetAllActorsOfClass` "/Script/Engine.PlayerStart"))
      (set `self.GM_SpawnPoints` _outactors))))

(event `Link Menu UI to GM`
  (params (CurrentUI :type "UserWidget Object Reference"))
  ;[1 1 1] Linking UI to this Gamemode so it can change the button selection
  (set `self.UI_CurrentUI` CurrentUI))

(event `MenuAreaChange`
  (params (GameAreaName :type String))
  ;[1 1 1] Change area name function
  (bind _output_get (set `self._GameArea_` GameAreaName))
  (switch `string` _output_get
    (:`CharacterSelect`
      ;[1 1 1] Getting the character selection slots for movement later
      (bind _ascharacter_select (cast `/Game/UI/Menu/CharacterSelect` (`self.UI_CurrentUI`)))
      (set `self.UI_CharacterSelectSlots` (`|MakeArray` (`/Game/UI/Menu/CharacterSelect.Player1Mark` _ascharacter_select) (`/Game/UI/Menu/CharacterSelect.Player2Mark` _ascharacter_select) (`/Game/UI/Menu/CharacterSelect.Player3Mark` _ascharacter_select) (`/Game/UI/Menu/CharacterSelect.Player4Mark` _ascharacter_select))))))

(event `SpawnCharacter`
  (params (`Player Controller` :type "PlayerController Object Reference"))
  (bind _returnvalue (`Controller.K2_GetPawn` `Player Controller`))
  ;[1 1 1] Deleting the spectator pawn, and creating a player pawn for them to possess
  (`self.PreSpawnCharacterChecks` `Player Controller`)
  (`/Engine/EditorBlueprintResources/StandardMacros.IsValid` _returnvalue
    (:`Is Valid`
      (`self.K2_DestroyActor` _returnvalue)
      (bind _characterbp (`self.AssignCharacter` `Player Controller`))
      (bind _returnvalue_2 (`|SpawnActorFromClass` _characterbp (`self.GetTransform` (`|GetArrayItem` (`self.GM_SpawnPoints`) (`GameplayStatics.GetPlayerControllerID` `Player Controller`))) "Undefined" "OverrideRootScale" null null))
      (`Controller.Possess` `Player Controller` _returnvalue_2)
      (`PlayerController.SetViewTargetWithBlend` `Player Controller` (`self.GameCamera`) 0.0 "VTBlend_Linear" 0.0 false)
      (set `/Game/BluePrints/PlayerBP/DEFAULT_PLAYER_BP.CurrentController` `Player Controller` _returnvalue_2)
      (`self.DisableInput` _returnvalue_2 `Player Controller`))))

(event `GM_MenuUp`
  (params (PlayerController :type "PlayerController Object Reference"))
  (bind _returnvalue (`GameplayStatics.GetPlayerControllerID` PlayerController))
  (bind _ui_menubuttonindexmultiplayer (`self.UI_MenuButtonIndexMultiplayer`))
  (switch `string` (`self._GameArea_`)
    (:`MainMenuLevel`
      ;[1 1 1] Updating Index and UI selection on button press
      (bind _newindex (`self.CheckForOutOfBounds` (- (`self.UI_MenuButtonIndex`) 1) 4))
      (bind _output_get (set `self.UI_MenuButtonIndex` _newindex))
      (bind _asmain_menu_ui (cast `/Game/UI/Menu/MainMenuUI` (`self.UI_CurrentUI`)))
      (`/Game/UI/Menu/MainMenuUI.UpdateSelection` _asmain_menu_ui _output_get))
    (:`CharacterSelect`
      (bind _newindex_2 (`self.CheckForOutOfBounds` (- (`|GetArrayItem` _ui_menubuttonindexmultiplayer _returnvalue) 1) 3))
      (`KismetArrayLibrary.Array_Set` _ui_menubuttonindexmultiplayer _returnvalue _newindex_2)
      (`self.MoveCharacterSelectIcon` _returnvalue _newindex_2 (`self.CS_PlayerCharacterHovered`)))))

(event `DespawnCharacter`
  (params (`Player Controller` :type "PlayerController Object Reference"))
  (bind _returnvalue (`Controller.K2_GetPawn` `Player Controller`))
  ;[1 1 1] Deleting the player pawn and creating a spectator pawn for them to possess
  (`/Engine/EditorBlueprintResources/StandardMacros.IsValid` _returnvalue
    (:`Is Valid`
      (`self.K2_DestroyActor` _returnvalue)
      (bind _returnvalue_2 (`|SpawnActorFromClass` "/Game/BluePrints/PlayerBP/SpectatorTest.SpectatorTest_C" (`self.GetTransform` (`|GetArrayItem` (`self.GM_SpawnPoints`) (`GameplayStatics.GetPlayerControllerID` `Player Controller`))) "Undefined" "OverrideRootScale" null null))
      (`Controller.Possess` `Player Controller` _returnvalue_2)
      (`PlayerController.SetViewTargetWithBlend` `Player Controller` (`self.GameCamera`) 0.0 "VTBlend_Linear" 0.0 false)
      (`KismetArrayLibrary.Array_Set` (`self.GM_PlayerActive`) (`GameplayStatics.GetPlayerControllerID` `Player Controller`)))))

(event `GM_MenuDown`
  (params (PlayerController :type "PlayerController Object Reference"))
  (bind _returnvalue (`GameplayStatics.GetPlayerControllerID` PlayerController))
  (bind _ui_menubuttonindexmultiplayer (`self.UI_MenuButtonIndexMultiplayer`))
  (switch `string` (`self._GameArea_`)
    (:`MainMenuLevel`
      ;[1 1 1] Updating Index and UI selection on button press
      (bind _newindex (`self.CheckForOutOfBounds` (+ (`self.UI_MenuButtonIndex`) 1) 4))
      (bind _output_get (set `self.UI_MenuButtonIndex` _newindex))
      (bind _asmain_menu_ui (cast `/Game/UI/Menu/MainMenuUI` (`self.UI_CurrentUI`)))
      (`/Game/UI/Menu/MainMenuUI.UpdateSelection` _asmain_menu_ui _output_get))
    (:`CharacterSelect`
      (bind _newindex_2 (`self.CheckForOutOfBounds` (+ (`|GetArrayItem` _ui_menubuttonindexmultiplayer _returnvalue) 1) 3))
      (`KismetArrayLibrary.Array_Set` _ui_menubuttonindexmultiplayer _returnvalue _newindex_2)
      (`self.MoveCharacterSelectIcon` _returnvalue _newindex_2 (`self.CS_PlayerCharacterHovered`)))))

(event `GM_MenuRight`
  (params (`Player Controller` :type "PlayerController Object Reference"))
  (bind _returnvalue (`GameplayStatics.GetPlayerControllerID` `Player Controller`))
  (bind _cs_playercharacterhovered (`self.CS_PlayerCharacterHovered`))
  (bind _output (`|GetArrayItem` (`self.UI_MenuButtonIndexMultiplayer`) (`GameplayStatics.GetPlayerControllerID` `Player Controller`)))
  (switch `string` (`self._GameArea_`)
    (:`CharacterSelect`
      ;[1 1 1] Check if the player is hovering over the characters
      (if (== _output 0)
        ;[1 1 1] Changing character Right
        (bind _newindex (`self.CheckForOutOfBounds` (+ (`|GetArrayItem` _cs_playercharacterhovered _returnvalue) 1) (`KismetArrayLibrary.Array_Length` (`self.CS_ListOfPlayableCharacter`))))
        (`KismetArrayLibrary.Array_Set` _cs_playercharacterhovered _returnvalue _newindex)
        ;[1 1 1] Update UI
        (`self.MoveCharacterSelectIcon` _returnvalue _output _cs_playercharacterhovered)))))

(event `GM_MenuLeft`
  (params (`Player Controller` :type "PlayerController Object Reference"))
  (bind _returnvalue (`GameplayStatics.GetPlayerControllerID` `Player Controller`))
  (bind _cs_playercharacterhovered (`self.CS_PlayerCharacterHovered`))
  (bind _output (`|GetArrayItem` (`self.UI_MenuButtonIndexMultiplayer`) (`GameplayStatics.GetPlayerControllerID` `Player Controller`)))
  (switch `string` (`self._GameArea_`)
    (:`CharacterSelect`
      ;[1 1 1] Check if the player is hovering over the characters
      (if (== _output 0)
        ;[1 1 1] Changing character Right
        (bind _newindex (`self.CheckForOutOfBounds` (- (`|GetArrayItem` _cs_playercharacterhovered _returnvalue) 1) (`KismetArrayLibrary.Array_Length` (`self.CS_ListOfPlayableCharacter`))))
        (`KismetArrayLibrary.Array_Set` _cs_playercharacterhovered _returnvalue _newindex)
        ;[1 1 1] Update UI
        (`self.MoveCharacterSelectIcon` _returnvalue _output _cs_playercharacterhovered)))))

(event `self.ReceiveEndPlay`
  (params (EndPlayReason :type "EEndPlayReason Enum" :default "Destroyed"))
  (switch `string` (`self._GameArea_`)
    (:`CharacterSelect`
      ;[1 1 1] Updating game instance If we are leaving the character select
      (bind _asthe_game_instance (cast `/Game/THE_GAME_INSTANCE` (`GameplayStatics.GetGameInstance`)))
      (set `/Game/THE_GAME_INSTANCE.INSTANCE_PlayerActive` (`self.GM_PlayerActive`) _asthe_game_instance)
      (set `/Game/THE_GAME_INSTANCE.INSTANCE_PlayerCharacterSelected` (`self.CS_PlayerCharacterSelected`) _asthe_game_instance))))

(event `GM_TriggerRight`
  (params (`Player Controller` :type "PlayerController Object Reference"))
  (bind _returnvalue (`GameplayStatics.GetPlayerControllerID` `Player Controller`))
  (bind _ui_currentui (`self.UI_CurrentUI`))
  (bind _ui_menubuttonindexmultiplayer (`self.UI_MenuButtonIndexMultiplayer`))
  (bind _cs_readyplayers (`self.CS_ReadyPlayers`))
  (switch `string` (`self._GameArea_`)
    (:`MainMenuLevel`
      ;[1 1 1] Finalize selection for menu
      (bind _asmain_menu_ui (cast `/Game/UI/Menu/MainMenuUI` (`self.UI_CurrentUI`)))
      (`/Game/UI/Menu/MainMenuUI.IWantThatButtonPicked` _asmain_menu_ui)
      ;[1 1 1] Reseting selection
      (bind _output_get (set `self.UI_MenuButtonIndex` 0))
      (bind _asmain_menu_ui_2 (cast `/Game/UI/Menu/MainMenuUI` (`self.UI_CurrentUI`)))
      (`/Game/UI/Menu/MainMenuUI.UpdateSelection` _asmain_menu_ui_2 _output_get))
    (:`CharacterSelect`
      ;[1 1 1] Spawning the hovered character, or joining for the first time
      (if (`|GetArrayItem` (`self.GM_PlayerActive`) _returnvalue)
        (switch `int` (`|GetArrayItem` _ui_menubuttonindexmultiplayer _returnvalue)
          (:`0`
            ;[1 1 1] SpawnCharacterSelection
            (`self.SpawnCharacter` `Player Controller` :!label _label)
            (`self.MoveCharacterSelectIcon` _returnvalue 0 (`self.CS_PlayerCharacterHovered`)))
          (:`1`
            ;[1 1 1] Flip/Flop that players ready up status
            (if (`|GetArrayItem` _cs_readyplayers _returnvalue)
              (`KismetArrayLibrary.Array_Set` _cs_readyplayers _returnvalue)
              (bind _ascharacter_select (cast `/Game/UI/Menu/CharacterSelect` _ui_currentui))
              (`/Game/UI/Menu/CharacterSelect.PlayerReadyDown` _ascharacter_select _returnvalue)
              (else
                (`KismetArrayLibrary.Array_Set` _cs_readyplayers _returnvalue true)
                (bind _ascharacter_select_2 (cast `/Game/UI/Menu/CharacterSelect` _ui_currentui))
                (`/Game/UI/Menu/CharacterSelect.PlayerReadyUp` _ascharacter_select_2 _returnvalue)
                (bind _allready (`self.AreAllPlayersReady` (`self.GM_PlayerActive`) (`self.CS_ReadyPlayers`)))
                (if _allready
                  ;[1 0 0] CHANGE TO LEVEL SELECT
                  (`GameplayStatics.OpenLevel` "BaseLevel")))))
          (:`2`
            ;[1 1 1] Back to menu
            (bind _ascharacter_select_3 (cast `/Game/UI/Menu/CharacterSelect` (`self.UI_CurrentUI`)))
            (`/Game/UI/Menu/CharacterSelect.BackToMenu` _ascharacter_select_3)
            (set `self.UI_MenuButtonIndexMultiplayer` (`|MakeArray` 0 0 0 0))
            ;[1 1 1] Despawn all actors from screen
            (bind _outactors (`GameplayStatics.GetAllActorsOfClass` "/Script/Engine.PlayerController"))
            (for _array_element _outactors
              (if (and (`|GetArrayItem` (`self.GM_PlayerActive`) (`GameplayStatics.GetPlayerControllerID` _array_element)) (`KismetSystemLibrary.IsValid` (`Controller.K2_GetPawn` _array_element)))
                (`self.DespawnCharacter` _array_element)))))
        (else
          (`KismetArrayLibrary.Array_Set` _ui_menubuttonindexmultiplayer _returnvalue)
          (goto _label))))))

(event `GM_TriggerLeft`
  (params (`Player Controller` :type "PlayerController Object Reference"))
  (switch `string` (`self._GameArea_`)
    (:`CharacterSelect`
      ;[1 1 1] Despawn the character seleciton
      (`self.DespawnCharacter` `Player Controller`)
      (`self.MoveCharacterSelectIcon` (`GameplayStatics.GetPlayerControllerID` `Player Controller`) 0 (`self.CS_PlayerCharacterHovered`)))))

(fn `AreAllPlayersReady`
  (params (PlayersActive :type "Array of Boolean") (NewParam1 :type "Array of Boolean"))
  (returns (AllReady :type Boolean))
  (locals (PlayersReady :type Integer) (TotalPlayers :type Integer))
  (set `local.TotalPlayers` 0)
  (set `local.PlayersReady` 0)
  (for _array_element PlayersActive
    (if _array_element
      (set `local.TotalPlayers` (+ (`local.TotalPlayers`) 1))))
  (for _array_element_2 NewParam1
    (if _array_element_2
      (set `local.PlayersReady` (+ (`local.PlayersReady`) 1))))
  (if (== (`local.PlayersReady`) (`local.TotalPlayers`))
    (return true)
    (else
      (return false))))

(fn `AssignCharacter`
  (params (`Player Controller` :type "PlayerController Object Reference"))
  (returns (CharacterBP :type "/Game/BluePrints/PlayerBP/DEFAULT_PLAYER_BP Class Reference"))
  (bind _returnvalue (`GameplayStatics.GetPlayerControllerID` `Player Controller`))
  (bind _cs_playercharacterselected (`self.CS_PlayerCharacterSelected`))
  (bind _output (`|GetArrayItem` _cs_playercharacterselected _returnvalue))
  (if (> _output (- (`KismetArrayLibrary.Array_Length` _cs_playercharacterselected) 1))
    (`KismetArrayLibrary.Array_Set` _cs_playercharacterselected _returnvalue)
    (return (`|GetArrayItem` (`self.CS_ListOfPlayableCharacter`)))
    (else
      (return (`|GetArrayItem` (`self.CS_ListOfPlayableCharacter`) _output)))))

(fn `CheckForOutOfBounds`
  (params (Index :type Integer) (ArrayLength :type Integer))
  (returns (NewIndex :type Integer))
  (if (< Index 0)
    (return (- ArrayLength 1)) ; If smaller than 0, set to the last index
    (elif (>= Index ArrayLength)
      (return 0) ; If greater than or = to the length of the array, set to 0
      (else
        (return Index) ; If it's fine just return the value
      ))))

(fn `MoveCharacterSelectIcon`
  (params (ControllerID :type Integer) (MenuIndex :type Integer) (PlayerCharacterHovered :type "Array of Integer"))
  (locals (CharacterSelectP1Pos :type "Array of Vector2D Structure") (MenuSelectP1Pos :type "Array of Vector2D Structure") (CharacterSelectP2Pos :type "Array of Vector2D Structure") (MenuSelectP2Pos :type "Array of Vector2D Structure"))
  (bind _returnvalue (`WidgetLayoutLibrary.SlotAsCanvasSlot` (`|GetArrayItem` (`self.UI_CharacterSelectSlots`) ControllerID)))
  ;[1 1 1] If we're not active, put offscreen. If we are, put in a position based on thier index
  (if (`|GetArrayItem` (`self.GM_PlayerActive`) ControllerID)
    (if (== MenuIndex 0)
      (`CanvasPanelSlot.SetPosition` _returnvalue (`|GetArrayItem` (select `int` ControllerID :`0` (`local.CharacterSelectP1Pos`) :`1` (`local.CharacterSelectP2Pos`) :`2` _ :`3` _) (`|GetArrayItem` PlayerCharacterHovered ControllerID)))
      (else
        (`CanvasPanelSlot.SetPosition` (`WidgetLayoutLibrary.SlotAsCanvasSlot` (`|GetArrayItem` (`self.UI_CharacterSelectSlots`) ControllerID)) (`|GetArrayItem` (select `int` ControllerID :`0` (`local.MenuSelectP1Pos`) :`1` (`local.MenuSelectP2Pos`) :`2` _ :`3` _) MenuIndex))))
    (else
      (`CanvasPanelSlot.SetPosition` _returnvalue (0.0 5000.0)) ; OffScreen
    )))

(fn `PreSpawnCharacterChecks`
  (params (`Player controller` :type "PlayerController Object Reference"))
  (bind _returnvalue (`GameplayStatics.GetPlayerControllerID` `Player controller`))
  (switch `string` (`self._GameArea_`)
    (:`CharacterSelect`
      (`KismetArrayLibrary.Array_Set` (`self.GM_PlayerActive`) _returnvalue true)
      (`KismetArrayLibrary.Array_Set` (`self.CS_PlayerCharacterSelected`) _returnvalue (`|GetArrayItem` (`self.CS_PlayerCharacterHovered`) _returnvalue))
      (return))))

(fn `UserConstructionScript`)