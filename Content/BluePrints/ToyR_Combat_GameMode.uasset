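; Game mode for Toy Rumble's local multiplayer combat, running matches from spawn to last player standing.
; On BeginPlay it creates local players, reads joins and character picks from the game instance, and possesses spawned pawns on a shared camera.
; Deaths move controllers between alive and dead arrays; one survivor triggers GameState rankings, the end screen and timeline-driven slow motion.
; It also handles spectator despawning, time-dilation pausing with wraparound menu selection, and returning to the main menu.
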(event `self.ReceiveBeginPlay`
  (bind _ig_playersalive (`self.IG_PlayersAlive`))
  (`|ExecutionSequence`
    (:`then_0`
      ;[1 1 1] Create 4 players
      (`GameplayStatics.CreatePlayer` 1)
      (`GameplayStatics.CreatePlayer` 2)
      (`GameplayStatics.CreatePlayer` 3))
    (:`then_1`
      ;[1 1 1] Getting Character spawn points
      (bind _outactors (`GameplayStatics.GetAllActorsOfClass` "/Script/Engine.PlayerStart"))
      (set `self.GM_SpawnPoints` _outactors))
    (:`then_2`
      ;[1 1 1] read the variables from instance
      (if (`self.GM_PlayableLevel`)
        (bind _asthe_game_instance (cast `/Game/THE_GAME_INSTANCE` (`GameplayStatics.GetGameInstance`)))
        (set `self.IG_PlayerCharacterSelected` (`/Game/THE_GAME_INSTANCE.INSTANCE_PlayerCharacterSelected` _asthe_game_instance))
        (set `self.GM_PlayerActive` (`/Game/THE_GAME_INSTANCE.INSTANCE_PlayerActive` _asthe_game_instance))
        ;[1 1 1] Start game player status
        (bind _outactors_2 (`GameplayStatics.GetAllActorsOfClass` "/Script/Engine.PlayerController"))
        (set `self.IG_PlayersAlive` _outactors_2)
        (`KismetArrayLibrary.Array_Clear` (`self.IG_PlayersDead`))
        ;[1 1 1] Delete any players that haven't joined the game
        (for _array_element _ig_playersalive :!label _label
          (if (not (`|GetArrayItem` (`self.GM_PlayerActive`) (`GameplayStatics.GetPlayerControllerID` _array_element)))
            (`KismetArrayLibrary.Array_RemoveItem` _ig_playersalive _array_element)
            (goto _label)))))
    (:`then_3`
      ;[1 1 1] Spawn each player's selection
      (`KismetSystemLibrary.Delay` 0.0)
      (for _array_element_2 (`self.IG_PlayersAlive`)
        (`self.SpawnCharacter` _array_element_2)))))

(event `SpawnCharacter`
  (params (`Player Controller` :type "PlayerController Object Reference"))
  (bind _returnvalue (`Controller.K2_GetPawn` `Player Controller`))
  ;[1 1 1] Deleting the spectator pawn, and creating a player pawn for them to possess
  (`/Engine/EditorBlueprintResources/StandardMacros.IsValid` _returnvalue
    (:`Is Valid`
      (`self.K2_DestroyActor` _returnvalue)
      (bind _characterbp (`self.Assign Character` `Player Controller`))
      (bind _returnvalue_2 (`|SpawnActorFromClass` _characterbp (`self.GetTransform` (`|GetArrayItem` (`self.GM_SpawnPoints`) (`GameplayStatics.GetPlayerControllerID` `Player Controller`))) "Undefined" "OverrideRootScale" null null))
      (`Controller.Possess` `Player Controller` _returnvalue_2)
      (`PlayerController.SetViewTargetWithBlend` `Player Controller` (`self.GameCamera`) 0.0 "VTBlend_Linear" 0.0 false)
      (set `/Game/BluePrints/PlayerBP/DEFAULT_PLAYER_BP.CurrentController` `Player Controller` _returnvalue_2)
      (bind _astoy_rumble_combat_controller (cast `/Game/BluePrints/PlayerBP/ToyRumbleCombatController` `Player Controller`))
      (set `/Game/BluePrints/PlayerBP/ToyRumbleCombatController.ControlledPawn` _returnvalue_2 _astoy_rumble_combat_controller))))

(event `PlayerDied`
  (params (PlayerController :type "PlayerController Object Reference"))
  ;[1 1 1] Move from alive array to dead array
  (for _array_element (`self.IG_PlayersAlive`)
    (if (== _array_element PlayerController)
      (`KismetArrayLibrary.Array_RemoveItem` (`self.IG_PlayersAlive`) PlayerController)
      (`KismetArrayLibrary.Array_AddUnique` (`self.IG_PlayersDead`) PlayerController)
      ;[1 1 1] Check if there is one player remaining
      (if (== (`KismetArrayLibrary.Array_Length` (`self.IG_PlayersAlive`)) 1)
        (`self.OneStanding`)))))

(event `OneStanding`
  ;[1 1 1] Last man standing
  (`|ExecutionSequence`
    (:`then_0`
      ;[1 1 1] Sending to GameState who placed what
      (bind _astoy_rumble_game_state (cast `/Game/BluePrints/ToyRumbleGameState` (`GameplayStatics.GetGameState`)))
      (`/Game/BluePrints/ToyRumbleGameState.SetPlayerRanking` _astoy_rumble_game_state (`self.IG_PlayersAlive`))
      (`/Game/BluePrints/ToyRumbleGameState.SetPlayerRanking` _astoy_rumble_game_state (`self.IG_PlayersDead`))
      ;[1 1 1] Display on screen
      (`WidgetLayoutLibrary.RemoveAllWidgets`)
      (bind _returnvalue (`|CreateWidget` "/Game/UI/InGame/Level1_EndGame.Level1_EndGame_C"))
      (`UserWidget.AddToViewport` _returnvalue 0)
      (`Timeline|IgnoreTimeDialationDelay`
        (:`Finished`
          (set `self.IG_GameNaturalFinish` true))))
    (:`then_1`
      ;[1 1 1] Slow the world down
      (bind (_direction _timeslowing) (`Timeline|Timeline_0` :!via `PlayFromStart`)
        (:`Update`
          (`GameplayStatics.SetGlobalTimeDilation` _timeslowing))))))

(event `DespawnCharacter`
  (params (`Player Controller` :type "PlayerController Object Reference"))
  (bind _returnvalue (`Controller.K2_GetPawn` `Player Controller`))
  ;[1 1 1] Deleting the player pawn and creating a spectator pawn for them to possess
  (`/Engine/EditorBlueprintResources/StandardMacros.IsValid` _returnvalue
    (:`Is Valid`
      (`self.K2_DestroyActor` _returnvalue)
      (bind _returnvalue_2 (`|SpawnActorFromClass` "/Game/BluePrints/PlayerBP/SpectatorTest.SpectatorTest_C" (`self.GetTransform` (`|GetArrayItem` (`self.GM_SpawnPoints`) (`GameplayStatics.GetPlayerControllerID` `Player Controller`))) "Undefined" "OverrideRootScale" null null))
      (`Controller.Possess` `Player Controller` _returnvalue_2)
      (`PlayerController.SetViewTargetWithBlend` `Player Controller` (`self.GameCamera`) 0.0 "VTBlend_Linear" 0.0 false)
      (`KismetArrayLibrary.Array_Set` (`self.GM_PlayerActive`) (`GameplayStatics.GetPlayerControllerID` `Player Controller`)))))

(event `DoneWithGame`
  ;[1 1 1] send back to menu
  (`GameplayStatics.SetGlobalTimeDilation` 1.0)
  (if (`self.IG_GameNaturalFinish`)
    (`GameplayStatics.OpenLevel` "MainMenuLevel")))

(event `PlayerPause`
  ;[1 1 1] Pausing
  (`/Engine/EditorBlueprintResources/StandardMacros.FlipFlop`
    (:`A`
      (set `self.IG_GamePaused` true)
      (`GameplayStatics.SetGlobalTimeDilation` 0.0)
      (bind _returnvalue (`|CreateWidget` "/Game/UI/InGame/PauseMenu.PauseMenu_C"))
      (`UserWidget.AddToViewport` _returnvalue 0)
      (set `self.IG_MenuSelection` 0))
    (:`B`
      (set `self.IG_GamePaused` false)
      (`GameplayStatics.SetGlobalTimeDilation` 1.0)
      (`/Game/UI/InGame/PauseMenu.NoMorePauseScreen` _returnvalue))))

(event `MenuUp`
  ;[1 1 1] Pause menus stuff
  (if (`self.IG_GamePaused`)
    (bind _newindex (`self.Check for Out Of Bounds` (- (`self.IG_MenuSelection`) 1) 3))
    (bind _output_get (set `self.IG_MenuSelection` _newindex))
    (`/Game/UI/InGame/PauseMenu.UpdateSelection` (stale `PlayerPause` _returnvalue) _output_get)))

(event `MenuDown`
  ;[1 1 1] Pause menus stuff
  (if (`self.IG_GamePaused`)
    (bind _newindex (`self.Check for Out Of Bounds` (+ (`self.IG_MenuSelection`) 1) 3))
    (bind _output_get (set `self.IG_MenuSelection` _newindex))
    (`/Game/UI/InGame/PauseMenu.UpdateSelection` (stale `PlayerPause` _returnvalue) _output_get)))

(event `MenuPickThat`
  ;[1 1 1] Pause menus stuff
  (if (`self.IG_GamePaused`)
    (`/Game/UI/InGame/PauseMenu.PickThatSelection` (stale `PlayerPause` _returnvalue) (`self.IG_MenuSelection`))))

(fn `Assign Character`
  (params (`Player contrller` :type "PlayerController Object Reference"))
  (returns (CharacterBP :type "/Game/BluePrints/PlayerBP/DEFAULT_PLAYER_BP Class Reference"))
  (bind _returnvalue (`GameplayStatics.GetPlayerControllerID` `Player contrller`))
  (bind _ig_playercharacterselected (`self.IG_PlayerCharacterSelected`))
  (bind _output (`|GetArrayItem` _ig_playercharacterselected _returnvalue))
  (if (> _output (- (`KismetArrayLibrary.Array_Length` _ig_playercharacterselected) 1))
    (`KismetArrayLibrary.Array_Set` _ig_playercharacterselected _returnvalue)
    (return (`|GetArrayItem` (`self.IG_ListOfPlayableCharacter`)))
    (else
      (return (`|GetArrayItem` (`self.IG_ListOfPlayableCharacter`) _output)))))

(fn `Check for Out Of Bounds`
  (params (Index :type Integer) (ArrayLength :type Integer))
  (returns (NewIndex :type Integer))
  (if (< Index 0)
    (return (- ArrayLength 1)) ; If smaller than 0, set to the last index
    (elif (>= Index ArrayLength)
      (return 0) ; If greater than or = to the length of the array, set to 0
      (else
        (return Index) ; If it's fine just return the value
      ))))

(fn `UserConstructionScript`)