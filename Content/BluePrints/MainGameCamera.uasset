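; MainGameCamera is a shared game camera that follows every actor tagged "Player" on a spring arm.
; Each tick it refreshes the player list and eases its root toward their average location, or toward a waiting point when none are found.
; While players exist, it also eases the spring arm's world rotation toward a target that starts at a default and is changed through the ChangeRotation event.
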(event `self.ReceiveBeginPlay`
  (bind _defaultrotation (`self.DefaultRotation`))
  (bind _outactors (`GameplayStatics.GetAllActorsWithTag` "Player"))
  (set `self.ListOfPlayers` _outactors)
  (set `self.NewRotation` _defaultrotation)
  (set `self.CurrentRotation` _defaultrotation))

(event `self.ReceiveTick`
  (params (DeltaSeconds :type "Float (single-precision)"))
  (bind _listofplayers (`self.ListOfPlayers`))
  (bind _root (`self.Root`))
  (bind _returnvalue (`KismetMathLibrary.RInterpTo` (`self.CurrentRotation`) (`self.NewRotation`) DeltaSeconds 1.0))
  (bind _outactors (`GameplayStatics.GetAllActorsWithTag` "Player"))
  (bind _output_get (set `self.ListOfPlayers` _outactors))
  (if (`KismetArrayLibrary.Array_IsValidIndex` _output_get)
    (bind _returnvalue_2 (`GameplayStatics.GetActorArrayAverageLocation` _listofplayers))
    (if (not (<= (`KismetArrayLibrary.Array_Length` _listofplayers) 0))
      (`SceneComponent.K2_SetWorldLocation` (`self.Root`) (`KismetMathLibrary.VInterpTo` (`SceneComponent.K2_GetComponentLocation` (`self.Root`)) _returnvalue_2 DeltaSeconds 1.0) false true)
      (`SceneComponent.K2_SetWorldRotation` (`self.SpringArm`) _returnvalue false false)
      (set `self.CurrentRotation` _returnvalue))
    (else
      (`SceneComponent.K2_SetWorldLocation` _root (`KismetMathLibrary.VInterpTo` (`SceneComponent.K2_GetComponentLocation` _root) (`self.WaitingPoint`) DeltaSeconds 1.0) false true))))

(event `ChangeRotation`
  (params (NewRotation :type "Rotator Structure"))
  (set `self.NewRotation` NewRotation))

(fn `UserConstructionScript`)