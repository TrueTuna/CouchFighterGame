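; Player controller for Toy Rumble that routes each player's input to either the menus or the controlled fighter.
; On BeginPlay it caches the menus game mode and the player pawn.
; Directional menu inputs always go to the game mode with the controller as sender.
; Abilities, attack and block reach the pawn only in playable levels; otherwise attack and block act as right and left menu triggers.
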(event `self.ReceiveBeginPlay`
  ;[1 1 1] GameMode cast
  (bind _astoy_r_menus_game_mode (cast `/Game/BluePrints/ToyR_Menus_GameMode` (`GameplayStatics.GetGameMode`)))
  (set `self.GameModeCast` _astoy_r_menus_game_mode)
  ;[1 1 1] Get controlled pawn
  (bind _asdefault_player_bp (cast `/Game/BluePrints/PlayerBP/DEFAULT_PLAYER_BP` (`self.K2_GetPawn` self)))
  (set `self.ControlledPawn` _asdefault_player_bp))

(event `InputAction|MenuUp`
  (params (Key :type "Key Structure"))
  ;[1 1 1] Menu Navigation
  (:`Pressed`
    (`/Game/BluePrints/ToyR_Menus_GameMode.GM_MenuUp` (`self.GameModeCast`) self)))

(event `InputAction|Ability1`
  (params (Key :type "Key Structure"))
  (:`Pressed`
    (if (`/Game/BluePrints/ToyR_Menus_GameMode.GM_PlayableLevel` (`self.GameModeCast`))
      (`/Game/BluePrints/PlayerBP/DEFAULT_PLAYER_BP.Ability1Pressed` (`self.ControlledPawn`)))))

(event `InputAction|MenuDown`
  (params (Key :type "Key Structure"))
  ;[1 1 1] Menu Navigation
  (:`Pressed`
    (`/Game/BluePrints/ToyR_Menus_GameMode.GM_MenuDown` (`self.GameModeCast`) self)))

(event `InputAction|MenuRight`
  (params (Key :type "Key Structure"))
  ;[1 1 1] Menu Navigation
  (:`Pressed`
    (`/Game/BluePrints/ToyR_Menus_GameMode.GM_MenuRight` (`self.GameModeCast`) self)))

(event `InputAction|Ability2`
  (params (Key :type "Key Structure"))
  (:`Pressed`
    (if (`/Game/BluePrints/ToyR_Menus_GameMode.GM_PlayableLevel` (`self.GameModeCast`))
      (`/Game/BluePrints/PlayerBP/DEFAULT_PLAYER_BP.Ability2Pressed` (`self.ControlledPawn`)))))

(event `InputAction|MenuLeft`
  (params (Key :type "Key Structure"))
  ;[1 1 1] Menu Navigation
  (:`Pressed`
    (`/Game/BluePrints/ToyR_Menus_GameMode.GM_MenuLeft` (`self.GameModeCast`) self)))

(event `InputAction|BasicAttack`
  (params (Key :type "Key Structure"))
  (:`Pressed`
    (if (`/Game/BluePrints/ToyR_Menus_GameMode.GM_PlayableLevel` (`self.GameModeCast`))
      ;[1 1 1] In game attack
      (`/Game/BluePrints/PlayerBP/DEFAULT_PLAYER_BP.BasicAttackPressed` (`self.ControlledPawn`))
      (else
        ;[1 1 1] Menu controls
        (`/Game/BluePrints/ToyR_Menus_GameMode.GM_TriggerRight` (`self.GameModeCast`) self)))))

(event `InputAction|Block`
  (params (Key :type "Key Structure"))
  (bind _gamemodecast (`self.GameModeCast`))
  (bind _gm_playablelevel (`/Game/BluePrints/ToyR_Menus_GameMode.GM_PlayableLevel` _gamemodecast))
  (:`Pressed`
    (if _gm_playablelevel
      ;[1 1 1] In-game
      (`/Game/BluePrints/PlayerBP/DEFAULT_PLAYER_BP.InputBlockPressed` (`self.ControlledPawn`))
      (else
        ;[1 1 1] Menu controls
        (`/Game/BluePrints/ToyR_Menus_GameMode.GM_TriggerLeft` _gamemodecast self))))
  (:`Released`
    (if _gm_playablelevel
      ;[1 1 1] In-game
      (`/Game/BluePrints/PlayerBP/DEFAULT_PLAYER_BP.InputBlockReleased` (`self.ControlledPawn`)))))

(fn `UserConstructionScript`)