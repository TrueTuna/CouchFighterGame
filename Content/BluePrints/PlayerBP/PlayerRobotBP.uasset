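; Robot player character with a punch, a second melee ability and a DEFCON laser-eye ultimate.
; Melee inputs play montages with physical animation switched off, while activate events damage and stagger players overlapping each hurt box.
; During DEFCON, Tick slows movement and turning, box-traces from the eye socket, updates the beam and damages players in its path.
; EnemyHitList prevents repeat hits, clearing periodically during the laser so damage ticks.
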(event `self.BasicAttackPressed`
  ;[1 1 1] Playing punch animation
  (if (and (not (`self.IsRagdolled`)) (not (`self.Attacking`)))
    (set `self.Attacking` true)
    (`self.PhysicalAnimTrigger` false)
    (bind _returnvalue (`self.PlayAnimMontage` (`|GetArrayItem` (`self.AnimMontageArray`))))
    (`KismetSystemLibrary.Delay` (/ _returnvalue 1.5))
    (`self.PhysicalAnimTrigger` true)
    (set `self.Attacking` false)))

(event `self.Ability1Pressed`
  ;[1 1 1] Playing ability 1 anim
  (if (and (not (`self.IsRagdolled`)) (not (`self.Attacking`)))
    (set `self.Attacking` true)
    (`self.PhysicalAnimTrigger` false)
    (bind _returnvalue (`self.PlayAnimMontage` (`|GetArrayItem` (`self.AnimMontageArray`) 1)))
    (`KismetSystemLibrary.Delay` (/ _returnvalue 1.5))
    (`self.PhysicalAnimTrigger` true)
    (set `self.Attacking` false)))

(event `self.ReceiveBeginPlay`
  ;[1 1 1] BEGIN
  (`parent.ReceiveBeginPlay`)
  (set `self.PlayerShieldFX` "/Game/ParticlesBP/C1_Robot/Robot_Shield.Robot_Shield"))

(event `self.Ability2Pressed`
  (bind _mesh (`self.Mesh`))
  ;[1 1 1] Ultimate ability input
  (if (and (not (`self.IsRagdolled`)) (not (`self.Attacking`)))
    (set `self.Attacking` true)
    (`GameplayStatics.SpawnEmitterAttached` "/Game/ParticlesBP/C1_Robot/EyeBlinkInvertedParticle.EyeBlinkInvertedParticle" _mesh "eye_r")
    (`GameplayStatics.SpawnEmitterAttached` "/Game/ParticlesBP/C1_Robot/EyeBlinkInvertedParticle.EyeBlinkInvertedParticle" _mesh "eye_l")
    (`KismetSystemLibrary.Delay` 1.1)
    (set `self.DEFCON` true)
    (`KismetArrayLibrary.Array_Clear` (`self.EnemyHitList`))
    (bind _returnvalue (`GameplayStatics.SpawnEmitterAtLocation` "/Game/ParticlesBP/C1_Robot/P1_LaserEyes.P1_LaserEyes"))
    (set `self.DefconLaserRef` _returnvalue)
    (bind _returnvalue_2 (`GameplayStatics.SpawnEmitterAtLocation` "/Game/ParticlesBP/C1_Robot/LaserEyesOut.LaserEyesOut" (0.0 0.0 0.0) (struct) (2.0 2.0 2.0)))
    (set `self.LaserEyeOutput` _returnvalue_2)))

(event `self.ReceiveDestroyed`
  (bind _defconlaserref (`self.DefconLaserRef`))
  (bind _lasereyeoutput (`self.LaserEyeOutput`))
  ;[1 1 1] Upon being destroyed
  (`/Engine/EditorBlueprintResources/StandardMacros.DoOnce` false ; Because Im calling on destrory, it will destroy for multiple frames causing errors
    (:`Completed`
      (if (`KismetSystemLibrary.IsValid` _defconlaserref)
        (`ActorComponent.K2_DestroyComponent` _defconlaserref)
        (if (`KismetSystemLibrary.IsValid` _lasereyeoutput)
          (`ActorComponent.K2_DestroyComponent` _lasereyeoutput))))))

(event `self.ReceiveTick`
  (params (DeltaSeconds :type "Float (single-precision)"))
  (bind _lasereyeoutput (`self.LaserEyeOutput`))
  (bind _defconlaserref (`self.DefconLaserRef`))
  (bind _mesh (`self.Mesh`))
  (bind _defconlaserref_2 (`self.DefconLaserRef`))
  (bind _returnvalue (`SceneComponent.GetSocketLocation` _mesh "eye"))
  (bind _returnvalue_2 (`SceneComponent.GetRightVector` _mesh))
  (bind _charactermovement (`self.CharacterMovement`))
  (bind _returnvalue_3 (* _returnvalue_2 10000.0))
  (bind _returnvalue_4 (`KismetMathLibrary.FindLookAtRotation` _returnvalue_2 _returnvalue_3))
  (bind _returnvalue_5 (+ _returnvalue _returnvalue_3))
  (`parent.ReceiveTick` DeltaSeconds)
  (`|ExecutionSequence`
    (:`then_0`
      ;[1 1 1] Are we defcon?
      (if (`self.DEFCON`)
        ;[1 1 1] Character movement stuff
        (set `CharacterMovementComponent.RotationRate` (struct :`Yaw` 25.0) _charactermovement)
        (set `CharacterMovementComponent.MaxWalkSpeed` 50.0 _charactermovement)
        ;[1 1 1] Check defcon time
        (if (and (not (`self.IsRagdolled`)) (< (`self.DEFCON_Timer`) (`self._DEFCON_Duration`)))
          (set `self.Attacking` true)
          ;[1 1 1] Update defcon timer
          (set `self.DEFCON_Timer` (+ (`self.DEFCON_Timer`) (`GameplayStatics.GetWorldDeltaSeconds`)))
          ;[1 1 1] Check if it's time to reset the damage list
          (if (< (`self.DEFCON_TickTime`) (`self._DEFCON_TickDuration`))
            ;[1 1 1] If no, add time to tick. If yes, clear array
            (set `self.DEFCON_TickTime` (+ (`self.DEFCON_TickTime`) (`GameplayStatics.GetWorldDeltaSeconds`)))
            (else
              (`KismetArrayLibrary.Array_Clear` (`self.EnemyHitList`))
              (set `self.DEFCON_TickTime` 0.0)))
          (`|ExecutionSequence`
            (:`then_0`
              ;[1 1 1] Draw a line infront of the character's head
              (bind _outhits (`KismetSystemLibrary.BoxTraceMulti` _returnvalue _returnvalue_5 (10.0 10.0 10.0) (struct) "TraceTypeQuery1"))
              ;[1 1 1] Check if array even exists
              (`ParticleSystemComponent.SetBeamSourcePoint` _defconlaserref_2 0 _returnvalue 0)
              (`ParticleSystemComponent.SetBeamTargetPoint` _defconlaserref_2 0 _returnvalue_5 0)
              (if (`KismetArrayLibrary.Array_IsValidIndex` _outhits)
                (for (_array_element _array_index) _outhits
                  (bind (_bblockinghit _binitialoverlap _time _distance _location _impactpoint _normal _impactnormal _physmat _hitactor) (`GameplayStatics.BreakHitResult` _array_element))
                  ;[1 0.2198 0] Check if its the last element for blocking purposes
                  (if (and (not (`Actor.bGenerateOverlapEventsDuringLevelStreaming` _hitactor)) (== _array_index (`KismetArrayLibrary.Array_LastIndex` _outhits)))
                    (`ParticleSystemComponent.SetBeamTargetPoint` (`self.DefconLaserRef`) 0 _impactpoint 0)
                    (`GameplayStatics.SpawnEmitterAtLocation` "/Game/ParticlesBP/C1_Robot/LaserEyesHit.LaserEyesHit" _impactpoint _returnvalue_4)
                    (else
                      (bind (_bblockinghit_2 _binitialoverlap_2 _time_2 _distance_2 _location_2 _impactpoint_2 _normal_2 _impactnormal_2 _physmat_2 _hitactor_2 _hitcomponent) (`GameplayStatics.BreakHitResult` _array_element))
                      ;[1 1 1] Check actors hit to see if one of them is a player
                      (bind (_tagfound _tagname) (`self.CheckAttackTagList` _hitcomponent))
                      (if (and _tagfound (`PrimitiveComponent.bGenerateOverlapEvents` _hitcomponent))
                        (`GameplayStatics.SpawnEmitterAtLocation` "/Game/ParticlesBP/C1_Robot/LaserEyesHit.LaserEyesHit" _location_2 _returnvalue_4)
                        ;[1 1 1] Have we hit them before
                        (bind _have_we_hit_them (`self.HaveWeHitBefore` _hitactor_2 (`self.EnemyHitList`)))
                        (if (not _have_we_hit_them)
                          ;[1 1 1] Deal damage and stagger
                          (switch `name` _tagname
                            (:`PlayerHitBox`
                              (bind _asdefault_player_bp (cast `/Game/BluePrints/PlayerBP/DEFAULT_PLAYER_BP` _hitactor_2))
                              (`self.Health_TakeDamage` _asdefault_player_bp 5.0)
                              (`self.StaggerHit` _asdefault_player_bp 10.0 (`SceneComponent.K2_GetComponentLocation` (`self.CapsuleComponent`)) true))))))))))
            (:`then_1`
              ;[1 1 1] Move the laser eye output
              (if (`KismetSystemLibrary.IsValid` _lasereyeoutput)
                (`SceneComponent.K2_SetWorldLocationAndRotation` _lasereyeoutput _returnvalue _returnvalue_4 false false))))
          (else
            ;[1 1 1] Reset once defcon is done
            (set `self.DEFCON_Timer` 0.0)
            (set `self.DEFCON_TickTime` 0.0)
            (set `self.DEFCON` false)
            (set `self.Attacking` false)
            (if (`KismetSystemLibrary.IsValid` _defconlaserref)
              (`ActorComponent.K2_DestroyComponent` _defconlaserref)
              (`ActorComponent.K2_DestroyComponent` (`self.LaserEyeOutput`))
              (set `CharacterMovementComponent.RotationRate` (struct :`Yaw` 500.0) _charactermovement)
              (set `CharacterMovementComponent.MaxWalkSpeed` 600.0 _charactermovement))))))))

(event `BasicAttackCharge`
  (bind _hurtbox_basicattack (`self.HurtBox_BasicAttack`))
  ;[1 1 1] Spawn attack particle 1
  (bind _returnvalue (`|SpawnActorFromClass` "/Game/ParticlesBP/C1_Robot/P1_Attack1_Spawnable.P1_Attack1_Spawnable_C" (`SceneComponent.K2_GetComponentToWorld` _hurtbox_basicattack) "Undefined" "OverrideRootScale" null null))
  (`self.K2_AttachToComponent` _returnvalue _hurtbox_basicattack "pelvis" "SnapToTarget" "SnapToTarget" "SnapToTarget" true))

(event `BasicAttackActivate`
  (bind _hurtbox_basicattack (`self.HurtBox_BasicAttack`))
  ;[1 1 1] Basic attacks Start
  (`ActorComponent.Activate` _hurtbox_basicattack false)
  (set `PrimitiveComponent.bGenerateOverlapEvents` true _hurtbox_basicattack)
  (`KismetArrayLibrary.Array_Clear` (`self.EnemyHitList`))
  (`|ExecutionSequence`
    (:`then_0`
      ;[1 1 1] Spawn attack particle 2
      (`GameplayStatics.SpawnEmitterAtLocation` "/Game/ParticlesBP/C1_Robot/P1_Attack1_2.P1_Attack1_2" (.location (`SceneComponent.K2_GetComponentToWorld` (`self.HurtBox_BasicAttack`))) (.rotation (`SceneComponent.K2_GetComponentToWorld` (`self.HurtBox_BasicAttack`)))))
    (:`then_1`
      ;[1 1 1] Add owner to the list so they can't get hit by their own attack
      (`KismetArrayLibrary.Array_Add` (`self.EnemyHitList`) (`KismetStringLibrary.Conv_StringToName` (`KismetSystemLibrary.GetObjectName` (`ActorComponent.GetOwner` (`self.HurtBox_BasicAttack`)))))
      ;[1 1 1] Check if the attack box hits a player's hitbox
      (for _array_element (`PrimitiveComponent.GetOverlappingComponents` (`self.HurtBox_BasicAttack`))
        (bind (_tagfound _tagname) (`self.CheckAttackTagList` _array_element))
        (if _tagfound
          (bind _returnvalue (`ActorComponent.GetOwner` _array_element))
          ;[1 1 1] Have we hit them before
          (bind _have_we_hit_them (`self.HaveWeHitBefore` _returnvalue (`self.EnemyHitList`)))
          (if (not _have_we_hit_them)
            ;[1 1 1] Deal damage and stagger
            (switch `name` _tagname
              (:`PlayerHitBox`
                (bind _asdefault_player_bp (cast `/Game/BluePrints/PlayerBP/DEFAULT_PLAYER_BP` _returnvalue))
                (`self.Health_TakeDamage` _asdefault_player_bp 10.0)
                (`self.StaggerHit` _asdefault_player_bp 10.0 (`SceneComponent.K2_GetComponentLocation` (`self.CapsuleComponent`)) true)))))))))

(event `BasicAttackDeactivate`
  ;[1 1 1] Basic attacks Start
  (`ActorComponent.Deactivate` (`self.HurtBox_BasicAttack`)))

(event `Ability1Activate`
  (bind _hurtbox_ability1 (`self.HurtBox_Ability1`))
  ;[1 1 1] Ability 1 Start
  (`ActorComponent.Activate` _hurtbox_ability1 false)
  (set `PrimitiveComponent.bGenerateOverlapEvents` true _hurtbox_ability1)
  (`KismetArrayLibrary.Array_Clear` (`self.EnemyHitList`))
  (`|ExecutionSequence`
    (:`then_0`
      ;[1 1 1] Spawn attack particle
      (`GameplayStatics.SpawnEmitterAtLocation` "/Game/ParticlesBP/C1_Robot/P1_Ability1.P1_Ability1" (.location (`SceneComponent.K2_GetComponentToWorld` (`self.HurtBox_Ability1`))) (.rotation (`SceneComponent.K2_GetComponentToWorld` (`self.HurtBox_Ability1`)))))
    (:`then_1`
      ;[1 1 1] Add owner to list
      (`KismetArrayLibrary.Array_Add` (`self.EnemyHitList`) (`KismetStringLibrary.Conv_StringToName` (`KismetSystemLibrary.GetObjectName` (`ActorComponent.GetOwner` (`self.HurtBox_Ability1`)))))
      ;[1 1 1] Check if we hit a component
      (for _array_element (`PrimitiveComponent.GetOverlappingComponents` (`self.HurtBox_Ability1`))
        (bind (_tagfound _tagname) (`self.CheckAttackTagList` _array_element))
        (if _tagfound
          (bind _returnvalue (`ActorComponent.GetOwner` _array_element))
          ;[1 1 1] Have we hit them before
          (bind _have_we_hit_them (`self.HaveWeHitBefore` _returnvalue (`self.EnemyHitList`)))
          (if (not _have_we_hit_them)
            ;[1 1 1] Ability 1 - Deal damage and stagger
            (switch `name` _tagname
              (:`PlayerHitBox`
                (bind _asdefault_player_bp (cast `/Game/BluePrints/PlayerBP/DEFAULT_PLAYER_BP` _returnvalue))
                (`self.Health_TakeDamage` _asdefault_player_bp 10.0)
                (`self.StaggerHit` _asdefault_player_bp 50.0 (`SceneComponent.K2_GetComponentLocation` (`self.CapsuleComponent`)) true)))))))))

(event `Ability1Deactivate`
  ;[1 1 1] Ability 1 Start
  (`ActorComponent.Deactivate` (`self.HurtBox_Ability1`)))

(fn `UserConstructionScript`
  (`parent.UserConstructionScript`))