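; Player controller for Toy Rumble that turns player input into join, leave and character selection requests.
; Each input event casts the game mode to ToyRumbleGameMode and passes this controller to it to spawn, despawn or cycle the character left or right.
; Joining and leaving only take effect when the game mode's PlayableLevel flag is false, while character switching has no such check.
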(event `InputAction|JoinGame`
  (params (Key :type "Key Structure"))
  (:`Pressed`
    (bind _astoy_rumble_game_mode (cast `/Game/BluePrints/ToyRumbleGameMode` (`GameplayStatics.GetGameMode`)))
    (if (not (`/Game/BluePrints/ToyRumbleGameMode.PlayableLevel` _astoy_rumble_game_mode))
      (`/Game/BluePrints/ToyRumbleGameMode.SpawnCharacter` _astoy_rumble_game_mode self))))

(event `InputAction|LeaveGame`
  (params (Key :type "Key Structure"))
  (:`Pressed`
    (bind _astoy_rumble_game_mode (cast `/Game/BluePrints/ToyRumbleGameMode` (`GameplayStatics.GetGameMode`)))
    (if (not (`/Game/BluePrints/ToyRumbleGameMode.PlayableLevel` _astoy_rumble_game_mode))
      (`/Game/BluePrints/ToyRumbleGameMode.DespawnCharacter` _astoy_rumble_game_mode self))))

(event `InputAction|CharacterRight`
  (params (Key :type "Key Structure"))
  (:`Pressed`
    (bind _astoy_rumble_game_mode (cast `/Game/BluePrints/ToyRumbleGameMode` (`GameplayStatics.GetGameMode`)))
    (`/Game/BluePrints/ToyRumbleGameMode.ChangeCharacterRight` _astoy_rumble_game_mode self)))

(event `InputAction|CharacterLeft`
  (params (Key :type "Key Structure"))
  (:`Pressed`
    (bind _astoy_rumble_game_mode (cast `/Game/BluePrints/ToyRumbleGameMode` (`GameplayStatics.GetGameMode`)))
    (`/Game/BluePrints/ToyRumbleGameMode.ChangeCharacterLeft` _astoy_rumble_game_mode self)))

(fn `UserConstructionScript`)