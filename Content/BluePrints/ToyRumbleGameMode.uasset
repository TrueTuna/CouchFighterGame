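; Game mode for Toy Rumble local multiplayer that creates extra players and handles character selection and pawn spawning.
; Spawn and despawn events swap spectator and character pawns at PlayerStarts indexed by controller ID, viewed through a shared GameCamera.
; Outside listed playable levels, players cycle characters with wraparound, and spawned characters have input disabled.
; Selections and active flags are saved to the game instance on EndPlay and restored in playable levels.
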(event `self.ReceiveBeginPlay`
  (`GameplayStatics.CreatePlayer` 1)
  (`GameplayStatics.CreatePlayer` 2)
  (`GameplayStatics.CreatePlayer` 3)
  ;[1 1 1] Getting Character spawn points'
  (bind _outactors (`GameplayStatics.GetAllActorsOfClass` "/Script/Engine.PlayerStart"))
  (set `self.SpawnPoints` _outactors)
  ;[1 1 1] Check if we are only a playable level
  (set `self.PlayableLevel` false)
  (bind _returnvalue (`GameplayStatics.GetCurrentLevelName` true))
  (for _array_element (`self.ListOfPlayableLevel`)
    (if (`KismetStringLibrary.EqualEqual_StrStr` _array_element _returnvalue)
      (set `self.PlayableLevel` true)
      ;[1 1 1] Setting all players to character 99 (Taken from INSTANCE)
      (bind _asthe_game_instance (cast `/Game/THE_GAME_INSTANCE` (`GameplayStatics.GetGameInstance`)))
      (set `self.PlayerCharacterSelected` (`/Game/THE_GAME_INSTANCE.INSTANCE_PlayerCharacterSelected` _asthe_game_instance))
      (set `self.PlayerActive` (`/Game/THE_GAME_INSTANCE.INSTANCE_PlayerActive` _asthe_game_instance)))))

(event `SpawnCharacter`
  (params (PlayerController :type "PlayerController Object Reference"))
  (bind _returnvalue (`Controller.K2_GetPawn` PlayerController))
  ;[1 1 1] Deleting the spectator pawn, and creating a player pawn for them to possess
  (`/Engine/EditorBlueprintResources/StandardMacros.IsValid` _returnvalue
    (:`Is Valid`
      (`self.K2_DestroyActor` _returnvalue)
      (bind _characterbp (`self.AssignCharacter` PlayerController))
      (bind _returnvalue_2 (`|SpawnActorFromClass` _characterbp (`self.GetTransform` (`|GetArrayItem` (`self.SpawnPoints`) (`GameplayStatics.GetPlayerControllerID` PlayerController))) "Undefined" "OverrideRootScale" null null))
      (`Controller.Possess` PlayerController _returnvalue_2)
      (`PlayerController.SetViewTargetWithBlend` PlayerController (`self.GameCamera`) 0.0 "VTBlend_Linear" 0.0 false)
      (set `/Game/BluePrints/PlayerRobotParentBP.CurrentController` PlayerController _returnvalue_2)
      (if (not (`self.PlayableLevel`))
        (`self.DisableInput` _returnvalue_2 PlayerController)
        (`KismetArrayLibrary.Array_Set` (`self.PlayerActive`) (`GameplayStatics.GetPlayerControllerID` PlayerController) true)))))

(event `DespawnCharacter`
  (params (PlayerController :type "PlayerController Object Reference"))
  (bind _returnvalue (`Controller.K2_GetPawn` PlayerController))
  ;[1 1 1] Deleting the player pawn and creating a spectator pawn for them to possess
  (`/Engine/EditorBlueprintResources/StandardMacros.IsValid` _returnvalue
    (:`Is Valid`
      (`self.K2_DestroyActor` _returnvalue)
      (bind _returnvalue_2 (`|SpawnActorFromClass` "/Game/BluePrints/SpectatorTest.SpectatorTest_C" (`self.GetTransform` (`|GetArrayItem` (`self.SpawnPoints`) (`GameplayStatics.GetPlayerControllerID` PlayerController))) "Undefined" "OverrideRootScale" null null))
      (`Controller.Possess` PlayerController _returnvalue_2)
      (`PlayerController.SetViewTargetWithBlend` PlayerController (`self.GameCamera`) 0.0 "VTBlend_Linear" 0.0 false)
      (`KismetArrayLibrary.Array_Set` (`self.PlayerActive`) (`GameplayStatics.GetPlayerControllerID` PlayerController)))))

(event `ChangeCharacterRight`
  (params (`Player Controller` :type "PlayerController Object Reference"))
  (bind _returnvalue (`GameplayStatics.GetPlayerControllerID` `Player Controller`))
  (bind _playercharacterselected (`self.PlayerCharacterSelected`))
  (bind _returnvalue_2 (+ (`|GetArrayItem` _playercharacterselected _returnvalue) 1))
  ;[1 1 1] Changing character Right
  (`/Engine/EditorBlueprintResources/StandardMacros.IsValid` (`Controller.K2_GetPawn` `Player Controller`)
    (:`Is Valid`
      (if (not (`self.PlayableLevel`))
        (if (> _returnvalue_2 (- (`KismetArrayLibrary.Array_Length` (`self.ListOfPlayableCharacter`)) 1))
          (`KismetArrayLibrary.Array_Set` _playercharacterselected _returnvalue)
          (else
            (`KismetArrayLibrary.Array_Set` _playercharacterselected _returnvalue _returnvalue_2)))
        (`self.SpawnCharacter` `Player Controller`)))))

(event `ChangeCharacterLeft`
  (params (`Player Controller` :type "PlayerController Object Reference"))
  (bind _returnvalue (`GameplayStatics.GetPlayerControllerID` `Player Controller`))
  (bind _playercharacterselected (`self.PlayerCharacterSelected`))
  (bind _returnvalue_2 (- (`|GetArrayItem` _playercharacterselected _returnvalue) 1))
  ;[1 1 1] Changing character left
  (`/Engine/EditorBlueprintResources/StandardMacros.IsValid` (`Controller.K2_GetPawn` `Player Controller`)
    (:`Is Valid`
      (if (not (`self.PlayableLevel`))
        (if (< _returnvalue_2 0)
          (`KismetArrayLibrary.Array_Set` _playercharacterselected _returnvalue (- (`KismetArrayLibrary.Array_Length` (`self.ListOfPlayableCharacter`)) 1))
          (else
            (`KismetArrayLibrary.Array_Set` _playercharacterselected _returnvalue _returnvalue_2)))
        (`self.SpawnCharacter` `Player Controller`)))))

(event `self.ReceiveEndPlay`
  (params (EndPlayReason :type "EEndPlayReason Enum" :default "Destroyed"))
  ;[1 1 1] Updating game instance
  (bind _asthe_game_instance (cast `/Game/THE_GAME_INSTANCE` (`GameplayStatics.GetGameInstance`)))
  (set `/Game/THE_GAME_INSTANCE.INSTANCE_PlayerActive` (`self.PlayerActive`) _asthe_game_instance)
  (set `/Game/THE_GAME_INSTANCE.INSTANCE_PlayerCharacterSelected` (`self.PlayerCharacterSelected`) _asthe_game_instance))

(fn `AssignCharacter`
  (params (`Player Controller` :type "PlayerController Object Reference"))
  (returns (CharacterBP :type "/Game/BluePrints/PlayerRobotParentBP Class Reference"))
  (bind _returnvalue (`GameplayStatics.GetPlayerControllerID` `Player Controller`))
  (bind _playercharacterselected (`self.PlayerCharacterSelected`))
  (bind _output (`|GetArrayItem` _playercharacterselected _returnvalue))
  (if (> _output (- (`KismetArrayLibrary.Array_Length` _playercharacterselected) 1))
    (`KismetArrayLibrary.Array_Set` _playercharacterselected _returnvalue)
    (return (`|GetArrayItem` (`self.ListOfPlayableCharacter`)))
    (else
      (return (`|GetArrayItem` (`self.ListOfPlayableCharacter`) _output)))))

(fn `UserConstructionScript`)