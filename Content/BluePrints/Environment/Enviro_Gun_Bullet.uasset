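; Environmental gun bullet projectile that damages and staggers player characters it overlaps.
; On spawn it launches its sphere with a large impulse along Direction, then destroys itself when LifeTime runs out.
; Its hitbox filters by component tag and records actor names in HitList to hit each player once.
; Stagger scales with Y/Z velocity, capped at a maximum and zeroed below a minimum, while health damage is a fixed amount.
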(event `self.ReceiveBeginPlay`
  ;[1 1 1] Spawning
  (`PrimitiveComponent.AddImpulse` (`self.Sphere`) (* (`self.Direction`) 600000) "None" false)
  (`KismetArrayLibrary.Array_Clear` (`self.HitList`)))

(event `self.ReceiveTick`
  (params (DeltaSeconds :type "Float (single-precision)"))
  ;[1 1 1] Lifetime check
  (bind _output_get (set `self.lifeTime` (- (`self.lifeTime`) DeltaSeconds)))
  (if (< _output_get 0.0)
    (`self.K2_DestroyActor`)))

(event `self.SphereHitbox.OnComponentBeginOverlap`
  (params (OverlappedComponent :type "PrimitiveComponent Object Reference") (OtherActor :type "Actor Object Reference") (OtherComp :type "PrimitiveComponent Object Reference") (OtherBodyIndex :type Integer) (bFromSweep :type Boolean) (SweepResult :type "HitResult Structure (by ref)"))
  (bind __maxstaggerdmg (`self._MaxStaggerDmg`))
  (bind _returnvalue (`KismetStringLibrary.Conv_StringToName` (`KismetSystemLibrary.GetObjectName` OtherActor)))
  ;[1 1 1] Overlapping with object
  (if (`ActorComponent.ComponentHasTag` OtherComp (`self.PlayerTagToLookFor`))
    ;[1 1 1] Check if we've already hit the object before
    (for _array_element (`self.HitList`)
      (if (== _returnvalue _array_element)
        (set `self.NameFound` true)))
    (if (not (`self.NameFound`))
      (`KismetArrayLibrary.Array_Add` (`self.HitList`) _returnvalue)
      ;[1 1 1] If hit is against Player
      (bind _asdefault_player_bp (cast `/Game/BluePrints/PlayerBP/DEFAULT_PLAYER_BP` OtherActor))
      (`|ExecutionSequence`
        (:`then_0`
          (bind _output_get (set `self.StaggerDamage` (* (`self.StaggerMulitplier`) (/ (`KismetMathLibrary.Hypotenuse` (.y (`SceneComponent.GetComponentVelocity` (`self.Sphere`))) (.z (`SceneComponent.GetComponentVelocity` (`self.Sphere`)))) 1000.0))))
          (if (> _output_get __maxstaggerdmg)
            (set `self.StaggerDamage` __maxstaggerdmg))
          (if (< _output_get (`self._MinStaggerDmg`))
            (set `self.StaggerDamage` 0.0))
          (`/Game/BluePrints/PlayerBP/DEFAULT_PLAYER_BP.StaggerHit` _asdefault_player_bp (`self.StaggerDamage`) (`self.K2_GetActorLocation`) false))
        (:`then_1`
          (`/Game/BluePrints/PlayerBP/DEFAULT_PLAYER_BP.Health_TakeDamage` _asdefault_player_bp 5.0))))))

(fn `UserConstructionScript`)