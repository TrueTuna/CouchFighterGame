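; Trigger area that changes the main game camera's angle while the camera is inside it.
; On BeginPlay it caches the level's MainGameCamera, assuming only one exists.
; When that camera begins overlapping, the area stores its DefaultRotation and calls ChangeRotation with the area's NewCameraRotation.
; When the overlap ends, it passes the stored rotation back to ChangeRotation to restore the default angle.
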(event `self.ReceiveBeginPlay`
  ;[1 1 1] Should only be one, so we get teh first one
  (bind _returnvalue (`GameplayStatics.GetActorOfClass` "/Game/BluePrints/MainGameCamera.MainGameCamera_C"))
  (set `self.MainGameCamera` _returnvalue))

(event `self.ReceiveActorBeginOverlap`
  (params (OtherActor :type "Actor Object Reference"))
  ;[1 1 1] Change camera angle when they enter
  (if (== OtherActor (`self.MainGameCamera`))
    (bind _asmain_game_camera (cast `/Game/BluePrints/MainGameCamera` OtherActor))
    (set `self.CameraDefaultRotation` (`/Game/BluePrints/MainGameCamera.DefaultRotation` _asmain_game_camera))
    (`/Game/BluePrints/MainGameCamera.ChangeRotation` _asmain_game_camera (`self.NewCameraRotation`))))

(event `self.ReceiveActorEndOverlap`
  (params (OtherActor :type "Actor Object Reference"))
  ;[1 1 1] Chnage camera angle back once it leave
  (if (== OtherActor (`self.MainGameCamera`))
    (bind _asmain_game_camera (cast `/Game/BluePrints/MainGameCamera` OtherActor))
    (`/Game/BluePrints/MainGameCamera.ChangeRotation` _asmain_game_camera (`self.CameraDefaultRotation`))))

(fn `UserConstructionScript`)