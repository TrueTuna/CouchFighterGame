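; Cat player character Blueprint with a melee basic attack and a timed phase ability; Ability 2 is an empty stub.
; Basic attack uses a placeholder timeline to check hurtbox overlaps once, applying stagger and damage to other players once each via a hit list.
; Phase disables hitboxes, boosts speed and swaps to a dynamic material.
; Tick flags Attacking during phase, then restores state and starts the cooldown.
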(event `self.ReceiveBeginPlay`
  ;[1 1 1] BEGIN
  (`parent.ReceiveBeginPlay`)
  (set `self._Ability1CoolDown_Duration` (`self.Cat_Ability1_CooldownDuration`))
  (set `self._Ability2CoolDown_Duration` (`self.Cat_Ability2_CooldownDuration`))
  ;[1 1 1] Materials
  (set `self.Cat_DefaultModelMaterial` "/Game/Materials/BuildingBlocks/Red.Red")
  (bind _returnvalue (`PrimitiveComponent.CreateDynamicMaterialInstance` (`self.Mesh`) 0 "/Game/Materials/Cat/PhaseAbility.PhaseAbility" "None"))
  (set `self.Cat_Ability1_PhaseMaterial` _returnvalue)
  (`PrimitiveComponent.SetMaterial` (`self.Mesh`) 0 (`self.Cat_DefaultModelMaterial`)))

(event `self.BasicAttackPressed`
  (bind _hurtbox_basicattack (`self.HurtBox_BasicAttack`))
  (`Timeline|Basic attack fake anim` :!via `PlayFromStart`
    (:`PretendAttackStart`
      ;[1 1 1] Hit detection
      (`ActorComponent.Activate` _hurtbox_basicattack false)
      (set `PrimitiveComponent.bGenerateOverlapEvents` true _hurtbox_basicattack)
      (`KismetArrayLibrary.Array_Clear` (`self.EnemyHitList`))
      ;[1 1 1] Add owner so they can't be hit by own attacks
      (`KismetArrayLibrary.Array_Add` (`self.EnemyHitList`) (`KismetStringLibrary.Conv_StringToName` (`KismetSystemLibrary.GetObjectName` (`ActorComponent.GetOwner` (`self.HurtBox_BasicAttack`)))))
      ;[1 1 1] Check if we hit a players hit box
      (for _array_element (`PrimitiveComponent.GetOverlappingComponents` (`self.HurtBox_BasicAttack`))
        (bind (_tagfound _tagname) (`self.CheckAttackTagList` _array_element))
        (if _tagfound
          (bind _returnvalue (`ActorComponent.GetOwner` _array_element))
          ;[1 1 1] Have we hit them before
          (bind _have_we_hit_them (`self.HaveWeHitBefore` _returnvalue (`self.EnemyHitList`)))
          (if (not _have_we_hit_them)
            ;[1 1 1] Deal damage and stagger
            (switch `name` _tagname
              (:`PlayerHitBox`
                (bind _asdefault_player_bp (cast `/Game/ActorBluePrints/PlayerBP/DEFAULT_PLAYER_BP` _returnvalue))
                (`self.StaggerHit` _asdefault_player_bp 10.0 (`SceneComponent.K2_GetComponentLocation` (`self.CapsuleComponent`)) 1.0)
                (`self.Health_TakeDamage` _asdefault_player_bp 10.0)))))))
    (:`PretendAttackEnd`
      (`ActorComponent.Deactivate` _hurtbox_basicattack))))

(event `self.BasicAttackActivate`)

(event `self.Ability1Pressed`
  ;[1 1 1] Checks
  (if (and (not (`self.Attacking`)) (<= (`self.Ability1CoolDown_Timer`) 0.0))
    ;[1 1 1] Disable hitboxes + speed boost
    (`PrimitiveComponent.SetCollisionProfileName` (`self.HitBox`) "NoCollision" true)
    (`PrimitiveComponent.SetCollisionProfileName` (`self.HitBoxArms`) "NoCollision" true)
    (`self.UpdateUnmodifiedMovespeed` 900.0)
    ;[1 1 1] Start timer
    (set `self.Ability1_UseTimer` (`self.Ability1_UseDuration`))
    ;[1 1 1] Visuals
    (`PrimitiveComponent.SetMaterial` (`self.Mesh`) 0 (`self.Cat_Ability1_PhaseMaterial`))
    ;[1 1 1] Event tick toggle
    (set `self.Ability1_Using` true)))

(event `self.Ability1Activate`)

(event `self.ReceiveTick`
  (params (DeltaSeconds :type "Float (single-precision)"))
  (`parent.ReceiveTick` DeltaSeconds)
  (`|ExecutionSequence`
    (:`then_0`
      ;[1 1 1] While ability 1 is active
      (if (`self.Ability1_Using`)
        (set `self.Attacking` true) ; Consume input
        (bind _output_get (set `self.Ability1_UseTimer` (- (`self.Ability1_UseTimer`) (`GameplayStatics.GetWorldDeltaSeconds`))))
        ;[1 1 1] Reset when time is up
        (if (<= _output_get 0.0)
          (set `self.Ability1_Using` false)
          (set `self.Attacking` false)
          (`self.UpdateUnmodifiedMovespeed` (`self._DefaultWalkSpeed_`))
          (`PrimitiveComponent.SetMaterial` (`self.Mesh`) 0 (`self.Cat_DefaultModelMaterial`))
          (`self.SetAbility1_OnCooldown` 1.0)
          (`PrimitiveComponent.SetCollisionProfileName` (`self.HitBox`) "OverlapAll" true)
          (`PrimitiveComponent.SetCollisionProfileName` (`self.HitBoxArms`) "OverlapAll" true))))))

(event `self.Ability2Pressed`)

(event `self.Ability2Activate`)

(event `self.ReceiveDestroyed`)

(fn `UserConstructionScript`
  (`parent.UserConstructionScript`))