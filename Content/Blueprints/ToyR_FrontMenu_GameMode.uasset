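; Front-menu game mode that creates extra local players on BeginPlay, for four in total, and relays menu input to the Menu_02 widget.
; Left and right change the character selection for the calling controller, and all four directions reset controller focus, while Accept is empty.
; The lockout timer counts down on Tick but only gates disconnected index-navigation logic.
; A helper function wraps out-of-range indices.
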(event `self.ReceiveBeginPlay`
  ;[1 1 1] BEGIN
  (`|ExecutionSequence`
    (:`then_0`
      ;[1 1 1] Create 4 players
      (`GameplayStatics.CreatePlayer` 1)
      (`GameplayStatics.CreatePlayer` 2)
      (`GameplayStatics.CreatePlayer` 3))))

(event `self.ReceiveTick`
  (params (DeltaSeconds :type "Float (single-precision)"))
  (`|ExecutionSequence`
    (:`then_0`
      ;[1 1 1] Countdown lockout timer
      (set `self.LockoutTimer` (- (`self.LockoutTimer`) DeltaSeconds)))))

(event `InputMenuUp`
  (bind _asmenu_02 (cast `/Game/UI/Menu_02/Menu_02` (`self.UIReference`) :!label _label))
  (`/Game/UI/Menu_02/Menu_02.ResetControllerFocus` _asmenu_02))

(event `InputMenuDown`
  (goto _label))

(event `InputMenuAccept`)

(event `InputMenuRight`
  (params (ControllerReference :type "PlayerController Object Reference"))
  ;[1 1 1] Tell
  (bind _asmenu_02 (cast `/Game/UI/Menu_02/Menu_02` (`self.UIReference`)))
  (`/Game/UI/Menu_02/Menu_02.Local_ChracterSelectChange_Right` _asmenu_02 ControllerReference)
  (goto _label))

(event `InputMenuLeft`
  (params (ControllerReference :type "PlayerController Object Reference"))
  ;[1 1 1] Tell
  (bind _asmenu_02 (cast `/Game/UI/Menu_02/Menu_02` (`self.UIReference`)))
  (`/Game/UI/Menu_02/Menu_02.Local_ChracterSelectChange_Left` _asmenu_02 ControllerReference)
  (goto _label))

(fn `CheckForOutOfBounds`
  (params (NumberOfItems :type Integer) (Index :type Integer))
  (returns (CleanedIndex :type Integer))
  (if (< Index 0)
    ;[1 1 1] Less than 0, set to the highest index
    (return (- NumberOfItems 1))
    (elif (>= Index NumberOfItems)
      ;[1 1 1] Greater than the legnth, set to 0
      (return 0)
      (else
        ;[1 1 1] Nothing wrong, nothing change
        (return Index)))))

(fn `UserConstructionScript`)