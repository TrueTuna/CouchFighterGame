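; Enviro_Gun_Physics is an environment gun that fires bullets automatically at a fixed interval.
; Tick accumulates elapsed time and, once FireSpeed has passed since the last shot, spawns an Enviro_Gun_Bullet at the Muzzle transform.
; Each bullet receives the Muzzle's forward vector as its Direction, and there is no targeting or trigger condition.
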(event `self.ReceiveBeginPlay`)

(event `self.ReceiveTick`
  (params (DeltaSeconds :type "Float (single-precision)"))
  (bind _muzzle (`self.Muzzle`))
  (bind _output_get (set `self.DeltaTimeTotal` (+ DeltaSeconds (`self.DeltaTimeTotal`))))
  (if (>= (- _output_get (`self.TimeSinceLastShot`)) (`self.FireSpeed`))
    (set `self.TimeSinceLastShot` _output_get)
    (`|SpawnActorFromClass` "/Game/Blueprints/Environment/Enviro_Gun_Bullet.Enviro_Gun_Bullet_C" (`SceneComponent.K2_GetComponentToWorld` _muzzle) "Undefined" "OverrideRootScale" null (`KismetMathLibrary.GetForwardVector` (`SceneComponent.K2_GetComponentRotation` _muzzle)) null)))

(fn `UserConstructionScript`)