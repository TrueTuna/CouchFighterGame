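; Menu game mode for up to four local players, routing directional and trigger inputs by current area: main menu, character select, level select or controls.
; It updates wrapping selection indices, drives the linked UI widget and moves the camera between tagged positions.
; Character select tracks joining, character choice and readiness per player, moving 3D icons between slots.
; When all are ready, a countdown opens level select and saves choices to the game instance.
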(event `GM_MenuUp`
  (params (PlayerController :type "PlayerController Object Reference"))
  (bind _returnvalue (`GameplayStatics.GetPlayerControllerID` PlayerController))
  (bind _ui_menubuttonindexmultiplayer (`self.UI_MenuButtonIndexMultiplayer`))
  (switch `string` (`self._GameArea_`)
    (:`MainMenuLevel`
      ;[1 1 1] Updating Index and UI selection on button press
      (bind _newindex (`self.Check for Out Of Bounds` (- (`self.UI_MenuButtonIndex`) 1) 4))
      (bind _output_get (set `self.UI_MenuButtonIndex` _newindex))
      (bind _asmain_menu_ui (cast `/Game/UI/Menu/MainMenuUI` (`self.UI_CurrentUI`)))
      (`/Game/UI/Menu/MainMenuUI.UpdateSelection` _asmain_menu_ui _output_get))
    (:`CharacterSelect`
      (bind _newindex_2 (`self.Check for Out Of Bounds` (- (`|GetArrayItem` _ui_menubuttonindexmultiplayer _returnvalue) 1) 2))
      (`KismetArrayLibrary.Array_Set` _ui_menubuttonindexmultiplayer _returnvalue _newindex_2)
      (`self.Update Character Select Icon` _returnvalue))
    (:`LevelSelect`
      (bind _newindex_3 (`self.Check for Out Of Bounds` (- (`self.UI_MenuButtonIndex`) 1) 2))
      (bind _output_get_2 (set `self.UI_MenuButtonIndex` _newindex_3))
      (bind _aslevel_select_ui (cast `/Game/UI/Menu/LevelSelectUI` (`self.UI_CurrentUI`)))
      (`/Game/UI/Menu/LevelSelectUI.UpdateButtons` _aslevel_select_ui _output_get_2)
      (`self.MoveLevelSelectIcon` _output_get_2 (`|GetArrayItem` (`self.UI_MenuButtonIndexMultiplayer`))))
    (:`Controls`
      (bind _newindex_4 (`self.Check for Out Of Bounds` (- (`self.UI_MenuButtonIndex`) 1) 3))
      (bind _output_get_3 (set `self.UI_MenuButtonIndex` _newindex_4))
      (bind _ascontrols_ui (cast `/Game/UI/Menu/ControlsUI` (`self.UI_CurrentUI`)))
      (`/Game/UI/Menu/ControlsUI.UpdateSelection` _ascontrols_ui _output_get_3))))

(event `self.ReceiveBeginPlay`
  (`|ExecutionSequence`
    (:`then_0`
      ;[1 1 1] Create 4 players
      (`GameplayStatics.CreatePlayer` 1)
      (`GameplayStatics.CreatePlayer` 2)
      (`GameplayStatics.CreatePlayer` 3))
    (:`then_1`
      ;[1 1 1] Set the level we are on
      (set `self._GameArea_` "CharacterSelect"))
    (:`then_2`
      ;[1 1 1] Getting Character spawn points (keep for character select)
      (bind _outactors (`GameplayStatics.GetAllActorsOfClass` "/Script/Engine.PlayerStart"))
      (set `self.GM_SpawnPoints` _outactors))
    (:`then_3`
      ;[1 1 1] Get camera positons
      (bind _outactors_2 (`GameplayStatics.GetAllActorsWithTag` "CameraPos"))
      (set `self.CameraPositions` _outactors_2))))

(event `Link Menu UI to GM`
  (params (CurrentUI :type "UserWidget Object Reference"))
  ;[1 1 1] Linking UI to this Gamemode so it can change the button selection
  (set `self.UI_CurrentUI` CurrentUI))

(event `MenuAreaChange`
  (params (GameAreaName :type String))
  ;[1 1 1] Change area name function
  (bind _output_get (set `self._GameArea_` GameAreaName))
  (switch `string` _output_get
    (:`MainMenuLevel`
      ;[1 1 1] Change camera pos
      (`self.K2_SetActorTransform` (`self.GameCamera`) (`self.GetTransform` (`|GetArrayItem` (`self.CameraPositions`))) false false))
    (:`CharacterSelect`
      ;[1 1 1] Getting the character selection slots for movement later
      (bind _outactors (`GameplayStatics.GetAllActorsWithTag` "CharacterSelectPos"))
      (set `self.3D_CharacterSlots` _outactors)
      ;[1 1 1] Get player slectors
      (bind _outactors_2 (`GameplayStatics.GetAllActorsWithTag` "PlayerSelectIcon"))
      (set `self.3D_PlayerObjs` _outactors_2)
      ;[1 1 1] Get menu selectors
      (bind _outactors_3 (`GameplayStatics.GetAllActorsWithTag` "CharacterMenuPos"))
      (set `self.3D_MenuSlots` _outactors_3)
      ;[1 1 1] Change camera pos
      (`self.K2_SetActorTransform` (`self.GameCamera`) (`self.GetTransform` (`|GetArrayItem` (`self.CameraPositions`) 1)) false false))
    (:`LevelSelect`
      ;[1 1 1] Getting level select slots for movement
      (bind _aslevel_select_ui (cast `/Game/UI/Menu/LevelSelectUI` (`self.UI_CurrentUI`)))
      (set `self.UI_SelectSlots` (`|MakeArray` (`/Game/UI/Menu/LevelSelectUI.UI_Level_Selector` _aslevel_select_ui) null null null))
      ;[1 1 1] Change camera pos
      (`self.K2_SetActorTransform` (`self.GameCamera`) (`self.GetTransform` (`|GetArrayItem` (`self.CameraPositions`) 2)) false false))))

(event `GM_MenuDown`
  (params (PlayerController :type "PlayerController Object Reference"))
  (bind _returnvalue (`GameplayStatics.GetPlayerControllerID` PlayerController))
  (bind _ui_menubuttonindexmultiplayer (`self.UI_MenuButtonIndexMultiplayer`))
  (switch `string` (`self._GameArea_`)
    (:`MainMenuLevel`
      ;[1 1 1] Updating Index and UI selection on button press
      (bind _newindex (`self.Check for Out Of Bounds` (+ (`self.UI_MenuButtonIndex`) 1) 4))
      (bind _output_get (set `self.UI_MenuButtonIndex` _newindex))
      (bind _asmain_menu_ui (cast `/Game/UI/Menu/MainMenuUI` (`self.UI_CurrentUI`)))
      (`/Game/UI/Menu/MainMenuUI.UpdateSelection` _asmain_menu_ui _output_get))
    (:`CharacterSelect`
      (bind _newindex_2 (`self.Check for Out Of Bounds` (+ (`|GetArrayItem` _ui_menubuttonindexmultiplayer _returnvalue) 1) 2))
      (`KismetArrayLibrary.Array_Set` _ui_menubuttonindexmultiplayer _returnvalue _newindex_2)
      (`self.Update Character Select Icon` _returnvalue))
    (:`LevelSelect`
      (bind _newindex_3 (`self.Check for Out Of Bounds` (+ (`self.UI_MenuButtonIndex`) 1) 2))
      (bind _output_get_2 (set `self.UI_MenuButtonIndex` _newindex_3))
      (bind _aslevel_select_ui (cast `/Game/UI/Menu/LevelSelectUI` (`self.UI_CurrentUI`)))
      (`/Game/UI/Menu/LevelSelectUI.UpdateButtons` _aslevel_select_ui _output_get_2)
      (`self.MoveLevelSelectIcon` _output_get_2 (`|GetArrayItem` (`self.UI_MenuButtonIndexMultiplayer`))))
    (:`Controls`
      (bind _newindex_4 (`self.Check for Out Of Bounds` (+ (`self.UI_MenuButtonIndex`) 1) 3))
      (bind _output_get_3 (set `self.UI_MenuButtonIndex` _newindex_4))
      (bind _ascontrols_ui (cast `/Game/UI/Menu/ControlsUI` (`self.UI_CurrentUI`)))
      (`/Game/UI/Menu/ControlsUI.UpdateSelection` _ascontrols_ui _output_get_3))))

(event `GM_MenuRight`
  (params (`Player Controller` :type "PlayerController Object Reference"))
  (bind _returnvalue (`GameplayStatics.GetPlayerControllerID` `Player Controller`))
  (bind _cs_playercharacterselected (`self.CS_PlayerCharacterSelected`))
  (switch `string` (`self._GameArea_`)
    (:`CharacterSelect`
      ;[1 1 1] Check if the player is hovering over the characters
      (if (and (== (`|GetArrayItem` (`self.CS_ReadyPlayers`) (`GameplayStatics.GetPlayerControllerID` `Player Controller`)) false) (== (`|GetArrayItem` (`self.UI_MenuButtonIndexMultiplayer`) (`GameplayStatics.GetPlayerControllerID` `Player Controller`)) 0))
        ;[1 1 1] Changing character Right
        (bind _newindex (`self.Check for Out Of Bounds` (+ (`|GetArrayItem` _cs_playercharacterselected _returnvalue) 1) (`KismetArrayLibrary.Array_Length` (`self.CS_ListOfPlayableCharacter`))))
        (`KismetArrayLibrary.Array_Set` _cs_playercharacterselected _returnvalue _newindex)
        (`self.Update Character Select Icon` _returnvalue)))
    (:`LevelSelect`
      ;[1 1 1] Funnel all inputs into player 1
      (bind _newindex_2 (`self.Check for Out Of Bounds` (+ (`|GetArrayItem` (`self.UI_MenuButtonIndexMultiplayer`)) 1) 4))
      (`KismetArrayLibrary.Array_Set` (`self.UI_MenuButtonIndexMultiplayer`) 0 _newindex_2)
      ;[1 1 1] Move buttons around
      (`self.MoveLevelSelectIcon` (`self.UI_MenuButtonIndex`) _newindex_2))
    (:`Controls`
      ;[1 1 1] Put volume slider right
      (if (== (`self.UI_MenuButtonIndex`) 1)
        (bind _ascontrols_ui (cast `/Game/UI/Menu/ControlsUI` (`self.UI_CurrentUI`)))
        (`/Game/UI/Menu/ControlsUI.VolumeRight` _ascontrols_ui)))))

(event `GM_MenuLeft`
  (params (`Player Controller` :type "PlayerController Object Reference"))
  (bind _returnvalue (`GameplayStatics.GetPlayerControllerID` `Player Controller`))
  (bind _cs_playercharacterselected (`self.CS_PlayerCharacterSelected`))
  (switch `string` (`self._GameArea_`)
    (:`CharacterSelect`
      ;[1 1 1] Check if the player is hovering over the characters
      (if (and (== (`|GetArrayItem` (`self.CS_ReadyPlayers`) (`GameplayStatics.GetPlayerControllerID` `Player Controller`)) false) (== (`|GetArrayItem` (`self.UI_MenuButtonIndexMultiplayer`) (`GameplayStatics.GetPlayerControllerID` `Player Controller`)) 0))
        ;[1 1 1] Changing character Right
        (bind _newindex (`self.Check for Out Of Bounds` (- (`|GetArrayItem` _cs_playercharacterselected _returnvalue) 1) (`KismetArrayLibrary.Array_Length` (`self.CS_ListOfPlayableCharacter`))))
        (`KismetArrayLibrary.Array_Set` _cs_playercharacterselected _returnvalue _newindex)
        (`self.Update Character Select Icon` _returnvalue)))
    (:`LevelSelect`
      ;[1 1 1] Funnel all inputs into player 1
      (bind _newindex_2 (`self.Check for Out Of Bounds` (- (`|GetArrayItem` (`self.UI_MenuButtonIndexMultiplayer`)) 1) 4))
      (`KismetArrayLibrary.Array_Set` (`self.UI_MenuButtonIndexMultiplayer`) 0 _newindex_2)
      ;[1 1 1] Move buttons around
      (`self.MoveLevelSelectIcon` (`self.UI_MenuButtonIndex`) _newindex_2))
    (:`Controls`
      ;[1 1 1] Put volume slider left
      (if (== (`self.UI_MenuButtonIndex`) 1)
        (bind _ascontrols_ui (cast `/Game/UI/Menu/ControlsUI` (`self.UI_CurrentUI`)))
        (`/Game/UI/Menu/ControlsUI.VolumeLeft` _ascontrols_ui)))))

(event `AllReadyCountdown`
  (bind _array (`|MakeArray` false false false false))
  (bind _ui_currentui (`self.UI_CurrentUI`))
  (bind (_direction _countdownvalue) (`Timeline|Countdown` :!via `PlayFromStart` :!label _label)
    (:`Finished`
      ;[1 1 1] Changing level
      (bind _ascharacter_select_ui (cast `/Game/UI/Menu/CharacterSelectUI` _ui_currentui))
      (`/Game/UI/Menu/CharacterSelectUI.GoToLevelSelect` _ascharacter_select_ui)
      ;[1 1 1] Updating game instance
      (bind _asthe_game_instance (cast `/Game/THE_GAME_INSTANCE` (`GameplayStatics.GetGameInstance`)))
      (set `/Game/THE_GAME_INSTANCE.INSTANCE_PlayerActive` (`self.GM_PlayerActive`) _asthe_game_instance)
      (set `/Game/THE_GAME_INSTANCE.INSTANCE_PlayerCharacterSelected` (`self.CS_PlayerCharacterSelected`) _asthe_game_instance)
      ;[1 1 1] Reset
      (set `self.UI_MenuButtonIndexMultiplayer` (`|MakeArray` 0 0 0 0))
      (set `self.UI_MenuButtonIndex` 0)
      (set `self.CS_ReadyPlayers` _array)
      (set `self.GM_PlayerActive` _array))
    (:`CountdownUpdate`
      ;[1 1 1] Update UI
      (bind _ascharacter_select_ui_2 (cast `/Game/UI/Menu/CharacterSelectUI` _ui_currentui))
      (`/Game/UI/Menu/CharacterSelectUI.UpdateCountdown` _ascharacter_select_ui_2 _countdownvalue))))

(event `AllReady_NOT`
  ;[1 1 1] Stop UI updates
  (bind _ascharacter_select_ui (cast `/Game/UI/Menu/CharacterSelectUI` (`self.UI_CurrentUI`)))
  (`/Game/UI/Menu/CharacterSelectUI.StopCountdown` _ascharacter_select_ui)
  (goto _label :!via `Stop`))

(event `GM_TriggerRight`
  (params (`Player Controller` :type "PlayerController Object Reference"))
  (bind _returnvalue (`GameplayStatics.GetPlayerControllerID` `Player Controller`))
  (bind _gm_playeractive (`self.GM_PlayerActive`))
  (bind _ui_currentui (`self.UI_CurrentUI`))
  (bind _ui_menubuttonindexmultiplayer (`self.UI_MenuButtonIndexMultiplayer`))
  (bind _gm_playeractive_2 (`self.GM_PlayerActive`))
  (switch `string` (`self._GameArea_`)
    (:`MainMenuLevel`
      ;[1 1 1] Finalize selection for menu
      (bind _asmain_menu_ui (cast `/Game/UI/Menu/MainMenuUI` (`self.UI_CurrentUI`)))
      (`/Game/UI/Menu/MainMenuUI.IWantThatButtonPicked` _asmain_menu_ui)
      (`KismetSystemLibrary.Delay` 0.9)
      ;[1 1 1] Reseting selection
      (bind _output_get (set `self.UI_MenuButtonIndex` 0))
      (bind _asmain_menu_ui_2 (cast `/Game/UI/Menu/MainMenuUI` (`self.UI_CurrentUI`)))
      (`/Game/UI/Menu/MainMenuUI.UpdateSelection` _asmain_menu_ui_2 _output_get))
    (:`CharacterSelect`
      ;[1 1 1] Selecting a character, or joining for the first time
      (if (`|GetArrayItem` _gm_playeractive_2 _returnvalue)
        (switch `int` (`|GetArrayItem` _ui_menubuttonindexmultiplayer _returnvalue)
          (:`0`
            ;[1 1 1] Turn on ready up for player
            (`KismetArrayLibrary.Array_Set` (`self.CS_ReadyPlayers`) _returnvalue true)
            (bind _ascharacter_select_ui (cast `/Game/UI/Menu/CharacterSelectUI` (`self.UI_CurrentUI`)))
            (`/Game/UI/Menu/CharacterSelectUI.PlayerReadyUp` _ascharacter_select_ui _returnvalue)
            (bind _allready (`self.AreAllPlayersReady` (`self.GM_PlayerActive`) (`self.CS_ReadyPlayers`)))
            (if _allready
              (`self.AllReadyCountdown`)))
          (:`1`
            ;[1 1 1] Cancel just in case
            (`self.AllReady_NOT`)
            ;[1 1 1] Back to menu
            (bind _ascharacter_select_ui_2 (cast `/Game/UI/Menu/CharacterSelectUI` (`self.UI_CurrentUI`)))
            (`/Game/UI/Menu/CharacterSelectUI.BackToMenu` _ascharacter_select_ui_2)
            (set `self.UI_MenuButtonIndexMultiplayer` (`|MakeArray` 0 0 0 0))
            ;[1 1 1] Unselect icons
            (`KismetSystemLibrary.Delay` 1.0)
            (for (_array_element _array_index) _gm_playeractive
              (if _array_element
                (`KismetArrayLibrary.Array_Set` _gm_playeractive _array_index)
                (`self.Update Character Select Icon` _array_index)))))
        (else
          (`KismetArrayLibrary.Array_Set` _ui_menubuttonindexmultiplayer _returnvalue)
          (`KismetArrayLibrary.Array_Set` _gm_playeractive_2 _returnvalue true)
          (`self.Update Character Select Icon` _returnvalue)
          (`self.AllReady_NOT`) ; Force cancel the countdown
        )))
    (:`LevelSelect`
      ;[1 1 1] Confiming selection
      (switch `int` (`self.UI_MenuButtonIndex`)
        (:`0`
          (bind _aslevel_select_ui (cast `/Game/UI/Menu/LevelSelectUI` _ui_currentui))
          (`/Game/UI/Menu/LevelSelectUI.ConfirmChoice` _aslevel_select_ui (`|GetArrayItem` (`self.UI_MenuButtonIndexMultiplayer`))))
        (:`1`
          (bind _aslevel_select_ui_2 (cast `/Game/UI/Menu/LevelSelectUI` _ui_currentui))
          (`/Game/UI/Menu/LevelSelectUI.Back` _aslevel_select_ui_2))))
    (:`Controls`
      ;[1 1 1] Finalize selection for menu
      (bind _ascontrols_ui (cast `/Game/UI/Menu/ControlsUI` (`self.UI_CurrentUI`)))
      (`/Game/UI/Menu/ControlsUI.IWantThatButtonPicked` _ascontrols_ui)
      ;[1 1 1] Only do when back button is pressed
      (if (== (`self.UI_MenuButtonIndex`) 2)
        ;[1 1 1] Reseting selection
        (bind _output_get_2 (set `self.UI_MenuButtonIndex` 0))
        (bind _asmain_menu_ui_3 (cast `/Game/UI/Menu/MainMenuUI` (`self.UI_CurrentUI`)))
        (`/Game/UI/Menu/MainMenuUI.UpdateSelection` _asmain_menu_ui_3 _output_get_2)))))

(event `GM_TriggerLeft`
  (params (`Player Controller` :type "PlayerController Object Reference"))
  (bind _returnvalue (`GameplayStatics.GetPlayerControllerID` `Player Controller`))
  (bind _gm_playeractive (`self.GM_PlayerActive`))
  (switch `string` (`self._GameArea_`)
    (:`CharacterSelect`
      ;[1 1 1] Check if player is ready
      (if (`|GetArrayItem` (`self.CS_ReadyPlayers`) _returnvalue)
        ;[1 1 1] Player is no longer ready
        (`self.AllReady_NOT`)
        (`KismetArrayLibrary.Array_Set` (`self.CS_ReadyPlayers`) _returnvalue)
        ;[1 1 1] UI turn off
        (bind _ascharacter_select_ui (cast `/Game/UI/Menu/CharacterSelectUI` (`self.UI_CurrentUI`)))
        (`/Game/UI/Menu/CharacterSelectUI.PlayerReadyDown` _ascharacter_select_ui _returnvalue)
        (else
          ;[1 1 1] If player is active, turn them off
          (if (`|GetArrayItem` _gm_playeractive _returnvalue)
            (`KismetArrayLibrary.Array_Set` _gm_playeractive _returnvalue)
            (`self.Update Character Select Icon` _returnvalue)))))))

(fn `AreAllPlayersReady`
  (params (PlayersActive :type "Array of Boolean") (PlayersReadyInput :type "Array of Boolean"))
  (returns (AllReady :type Boolean))
  (locals (PlayersReady :type Integer) (TotalPlayers :type Integer))
  (set `local.TotalPlayers` 0)
  (set `local.PlayersReady` 0)
  (for _array_element PlayersActive
    (if _array_element
      (set `local.TotalPlayers` (+ (`local.TotalPlayers`) 1))))
  (for _array_element_2 PlayersReadyInput
    (if _array_element_2
      (set `local.PlayersReady` (+ (`local.PlayersReady`) 1))))
  (if (== (`local.PlayersReady`) (`local.TotalPlayers`))
    (return true)
    (else
      (return false))))

(fn `AssignCharacter`
  (params (`Player Controller` :type "PlayerController Object Reference"))
  (returns (CharacterBP :type "/Game/Blueprints/PlayerBP/DEFAULT_PLAYER_BP Class Reference"))
  (bind _returnvalue (`GameplayStatics.GetPlayerControllerID` `Player Controller`))
  (bind _cs_playercharacterselected (`self.CS_PlayerCharacterSelected`))
  (bind _output (`|GetArrayItem` _cs_playercharacterselected _returnvalue))
  (if (> _output (- (`KismetArrayLibrary.Array_Length` _cs_playercharacterselected) 1))
    (`KismetArrayLibrary.Array_Set` _cs_playercharacterselected _returnvalue)
    (return (`|GetArrayItem` (`self.CS_ListOfPlayableCharacter`)))
    (else
      (return (`|GetArrayItem` (`self.CS_ListOfPlayableCharacter`) _output)))))

(fn `Check for Out Of Bounds`
  (params (Index :type Integer) (ArrayLength :type Integer))
  (returns (NewIndex :type Integer))
  (if (< Index 0)
    (return (- ArrayLength 1)) ; If smaller than 0, set to the last index
    (elif (>= Index ArrayLength)
      (return 0) ; If greater than or = to the length of the array, set to 0
      (else
        (return Index) ; If it's fine just return the value
      ))))

(fn `MoveLevelSelectIcon`
  (params (MenuIndex :type Integer) (LevelIndex :type Integer))
  (locals (LevelSelectPos :type "Array of Vector2D Structure") (MenuSelectPos :type "Array of Vector2D Structure"))
  (bind _returnvalue (`WidgetLayoutLibrary.SlotAsCanvasSlot` (`|GetArrayItem` (`self.UI_SelectSlots`))))
  (switch `int` MenuIndex
    (:`0`
      (`CanvasPanelSlot.SetPosition` _returnvalue (`|GetArrayItem` (`local.LevelSelectPos`) LevelIndex)) ; OffScreen
    )
    (:`1`
      (`CanvasPanelSlot.SetPosition` _returnvalue (`|GetArrayItem` (`local.MenuSelectPos`))) ; OffScreen
    )))

(fn `PreSpawnCharacterChecks`
  (params (`Player controller` :type "PlayerController Object Reference"))
  (bind _returnvalue (`GameplayStatics.GetPlayerControllerID` `Player controller`))
  (bind _cs_playercharacterselected (`self.CS_PlayerCharacterSelected`))
  (switch `string` (`self._GameArea_`)
    (:`CharacterSelect`
      (`KismetArrayLibrary.Array_Set` (`self.GM_PlayerActive`) _returnvalue true)
      (`KismetArrayLibrary.Array_Set` _cs_playercharacterselected _returnvalue (`|GetArrayItem` _cs_playercharacterselected _returnvalue))
      (return))))

(fn `Update Character Select Icon`
  (params (PlayerID :type Integer))
  (locals (CharacterSelectP1Pos :type "Array of Vector2D Structure") (MenuSelectP1Pos :type "Array of Vector2D Structure") (CharacterSelectP2Pos :type "Array of Vector2D Structure") (MenuSelectP2Pos :type "Array of Vector2D Structure"))
  (bind _output (`|GetArrayItem` (`self.UI_MenuButtonIndexMultiplayer`) PlayerID))
  ;[1 1 1] See if the person is even playing
  (if (`|GetArrayItem` (`self.GM_PlayerActive`) PlayerID)
    ;[1 1 1] Check if 0, 0 means character selector
    (if (== _output 0)
      ;[1 1 1] Get object and selection based on index, then move icon to position of character
      (`self.K2_SetActorTransform` (`|GetArrayItem` (`self.3D_PlayerObjs`) PlayerID) (`self.GetTransform` (`|GetArrayItem` (`self.3D_CharacterSlots`) (`|GetArrayItem` (`self.CS_PlayerCharacterSelected`) PlayerID))) false false)
      (else
        ;[1 1 1] Hovering the color over the selected menu
        (`self.K2_SetActorTransform` (`|GetArrayItem` (`self.3D_PlayerObjs`) PlayerID) (`self.GetTransform` (`|GetArrayItem` (`self.3D_MenuSlots`) (- _output 1))) false false)))
    (else
      ;[1 1 1] If player isnt playing
      (`self.K2_SetActorTransform` (`|GetArrayItem` (`self.3D_PlayerObjs`) PlayerID) (`KismetMathLibrary.MakeTransform` (0.0 0.0 -100.0) (struct) (0.1 0.1 0.1)) false false))))

(fn `UserConstructionScript`)