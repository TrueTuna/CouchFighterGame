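; Player controller for Toy Rumble combat that relays player input to its fighter and spawns the countdown widget.
; Movement, jump, attack, ability and block inputs forward to a ControlledPawn reference, though ability and block skip validity checks.
; Pause goes to the cached combat game mode.
; Tick retries that cache and re-applies the single MainGameCamera as view target every frame.
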(event `Set GamemodeCast`
  (params (GameMode :type "/Game/Blueprints/ToyR_Combat_GameMode Object Reference"))
  (set `self.GameModeCast` GameMode))

(event `self.ReceiveBeginPlay`
  (`/Engine/EditorBlueprintResources/StandardMacros.IsValid` (`self.GameModeCast`) :!label _label
    (:`Is Not Valid`
      ;[1 1 1] GameMode cast
      (bind _astoy_r_combat_game_mode (cast `/Game/Blueprints/ToyR_Combat_GameMode` (`GameplayStatics.GetGameMode`)))
      (set `self.GameModeCast` _astoy_r_combat_game_mode))))

(event `Controller_SpawnCountdown`
  ;[1 1 1] Widget countdown
  (bind _returnvalue (`|CreateWidget` "/Game/UI/Menu_02/Widgets/Countdown.Countdown_C" self))
  (`/Game/UI/Menu_02/Widgets/Countdown.ForcePlay` _returnvalue true)
  (`UserWidget.AddToViewport` _returnvalue 1))

(event `self.ReceiveTick`
  (params (DeltaSeconds :type "Float (single-precision)"))
  (`|ExecutionSequence`
    (:`then_0`
      (goto _label))
    (:`then_1`
      ;[1 1 1] Setting camera
      (`/Engine/EditorBlueprintResources/StandardMacros.IsValid` (`self.GameCamera`)
        (:`Is Valid`
          _)
        (:`Is Not Valid`
          (bind _outactors (`GameplayStatics.GetAllActorsOfClass` "/Game/Blueprints/PlayerBP/MainGameCamera.MainGameCamera_C"))
          (bind _output_get (set `self.GameCamera` (`|GetArrayItem` _outactors)))))
      (`self.SetViewTargetWithBlend` _output_get))))

(event `InputAction|PauseInGame` :paused true
  (params (Key :type "Key Structure"))
  ;[1 1 1] Menu Navigation
  (:`Pressed`
    (`/Game/Blueprints/ToyR_Combat_GameMode.PlayerPause` (`self.GameModeCast`))))

(event `InputAction|Ability1`
  (params (Key :type "Key Structure"))
  (:`Pressed`
    (if true
      (`/Game/Blueprints/PlayerBP/DEFAULT_PLAYER_BP.Ability1Pressed` (`self.ControlledPawn`)))))

(event `InputAction|MenuUp`
  (params (Key :type "Key Structure"))
  ;[1 1 1] Menu Navigation
)

(event `InputAction|MenuDown`
  (params (Key :type "Key Structure"))
  ;[1 1 1] Menu Navigation
)

(event `InputAction|Ability2`
  (params (Key :type "Key Structure"))
  (:`Pressed`
    (if true
      (`/Game/Blueprints/PlayerBP/DEFAULT_PLAYER_BP.Ability2Pressed` (`self.ControlledPawn`)))))

(event `InputAction|MenuRight`
  (params (Key :type "Key Structure"))
  ;[1 1 1] Menu Navigation
)

(event `InputAction|MenuLeft`
  (params (Key :type "Key Structure"))
  ;[1 1 1] Menu Navigation
)

(event `InputAction|BasicAttack`
  (params (Key :type "Key Structure"))
  (:`Pressed`
    ;[1 1 1] In game attack
    (`/Engine/EditorBlueprintResources/StandardMacros.IsValid` (`self.ControlledPawn`)
      (:`Is Valid`
        (`/Game/Blueprints/PlayerBP/DEFAULT_PLAYER_BP.BasicAttackPressed` (`self.ControlledPawn`))))))

(event `InputAxis|MoveForward`
  (params (AxisValue :type "Float (single-precision)"))
  (bind _controlledpawn (`self.ControlledPawn`))
  ;[1 1 1] Character Movement
  (`/Engine/EditorBlueprintResources/StandardMacros.IsValid` _controlledpawn
    (:`Is Valid`
      (`/Game/Blueprints/PlayerBP/DEFAULT_PLAYER_BP.MoveX` _controlledpawn AxisValue))))

(event `InputAxis|MoveRight`
  (params (AxisValue :type "Float (single-precision)"))
  (bind _controlledpawn (`self.ControlledPawn`))
  ;[1 1 1] Character Movement
  (`/Engine/EditorBlueprintResources/StandardMacros.IsValid` _controlledpawn
    (:`Is Valid`
      (`/Game/Blueprints/PlayerBP/DEFAULT_PLAYER_BP.MoveY` _controlledpawn AxisValue))))

(event `InputAction|Jump` :overrideparent false
  (params (Key :type "Key Structure"))
  (bind _controlledpawn (`self.ControlledPawn`))
  ;[1 1 1] CharacterJump
  (:`Pressed`
    (`/Engine/EditorBlueprintResources/StandardMacros.IsValid` _controlledpawn
      (:`Is Valid`
        (`/Game/Blueprints/PlayerBP/DEFAULT_PLAYER_BP.JumpPressed` _controlledpawn))))
  (:`Released`
    (`/Engine/EditorBlueprintResources/StandardMacros.IsValid` _controlledpawn
      (:`Is Valid`
        (`/Game/Blueprints/PlayerBP/DEFAULT_PLAYER_BP.JumpReleased` _controlledpawn)))))

(event `InputAction|Block`
  (params (Key :type "Key Structure"))
  (:`Pressed`
    (if true
      ;[1 1 1] In-game
      (`/Game/Blueprints/PlayerBP/DEFAULT_PLAYER_BP.InputBlockPressed` (`self.ControlledPawn`))))
  (:`Released`
    (if true
      ;[1 1 1] In-game
      (`/Game/Blueprints/PlayerBP/DEFAULT_PLAYER_BP.InputBlockReleased` (`self.ControlledPawn`)))))

(fn `OnRep_ControlledPawn`)

(fn `UserConstructionScript`)