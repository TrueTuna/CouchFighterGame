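; Playable Cat character with a melee basic attack, a phase ability and a summon, all triggered through authority-checked input events and gated by attack, ragdoll or cooldown state.
; The basic attack deals damage and stagger through a hurtbox overlap, with timelines blending montages against physical-animation ragdoll to prevent snapping.
; Phase disables hitboxes, swaps materials and boosts speed on a Tick timer.
; The summon roots the cat, then spawns three owner-tagged AI minions.
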(event `self.ReceiveBeginPlay`
  ;[1 1 1] BEGIN
  (`parent.ReceiveBeginPlay`)
  (set `self._Ability1CoolDown_Duration` (`self.Cat_Ability1_CooldownDuration`))
  (set `self._Ability2CoolDown_Duration` (`self.Cat_Ability2_CooldownDuration`))
  ;[1 1 1] Materials
  (set `self.Cat_DefaultModelMaterial` "/Game/Materials/Cat/Cat_BaseColour.Cat_BaseColour")
  (bind _returnvalue (`PrimitiveComponent.CreateDynamicMaterialInstance` (`self.Mesh`) 0 "/Game/Materials/Cat/PhaseAbilityOriginal.PhaseAbilityOriginal" "None"))
  (set `self.Cat_Ability1_PhaseMaterial` _returnvalue)
  (`PrimitiveComponent.SetMaterial` (`self.Mesh`) 0 (`self.Cat_DefaultModelMaterial`))
  ;[1 1 1] Bone Setting
  (set `self.PhysicalAnimationSettings` (make `PhysicalAnimationData` true 1000.0 10000.0 1000.0 1000.0))
  (set `self.ShieldBoneAttachPoint` "bn_pelvis01")
  (set `self.PhysicsStartPoint` "bn_neckA01")
  (`self.PhysicalAnimTrigger` true))

(event `self.Server_BasicAttackPressed`
  (bind _capsulecomponent (`self.CapsuleComponent`))
  (bind _hurtbox_basicattack (`self.HurtBox_BasicAttack`))
  (bind _returnvalue (`SceneComponent.GetForwardVector` _capsulecomponent))
  (bind _location (.location (`SceneComponent.K2_GetComponentToWorld` (`self.HurtBox_BasicAttack`))))
  (bind _x (.x (`SceneComponent.GetComponentVelocity` _capsulecomponent)))
  (bind _y (.y (`SceneComponent.GetComponentVelocity` _capsulecomponent)))
  ;[1 1 1] Checks
  (if (and (not (`self.Attacking`)) (not (`self.IsRagdolled`)))
    (set `self.Attacking` true)
    ;[1 1 1] Play real animation
    (`self.PlayAnimMontage` (`|GetArrayItem` (`self.AnimMontageArray`)))
    (bind (_direction _blendweight) (`Timeline|Basic attack fake anim` :!via `PlayFromStart`)
      (:`Update`
        (`self.PhysicalAnimTrigger` true _blendweight) ; Blend from animation to ragdoll to prevent snapping
      )
      (:`Finished`
        (`self.PhysicalAnimTrigger` true) ; Set back to ragdoll from animation
      )
      (:`PretendAttackStart`
        (`|ExecutionSequence`
          (:`then_0`
            ;[1 1 1] Spawn attack particle 2
            (`GameplayStatics.SpawnEmitterAtLocation` "/Game/ParticlesBP/Cat/CatBasicAttack_Particle.CatBasicAttack_Particle" (`KismetMathLibrary.MakeVector` (.x (select `bool` (or (> _x 300.0) (< _x -300.0) (> _y 300.0) (< _y -300.0)) :`false` (+ _location (* _returnvalue -30.0)) :`true` (+ (* _returnvalue 80.0) _location))) (.y (select `bool` (or (> _x 300.0) (< _x -300.0) (> _y 300.0) (< _y -300.0)) :`false` (+ _location (* _returnvalue -30.0)) :`true` (+ (* _returnvalue 80.0) _location))) (- (.z (select `bool` (or (> _x 300.0) (< _x -300.0) (> _y 300.0) (< _y -300.0)) :`false` (+ _location (* _returnvalue -30.0)) :`true` (+ (* _returnvalue 80.0) _location))) 50.0)) (`KismetMathLibrary.MakeRotator` (+ (.roll (.rotation (`SceneComponent.K2_GetComponentToWorld` (`self.HurtBox_BasicAttack`)))) 0.0) (.pitch (.rotation (`SceneComponent.K2_GetComponentToWorld` (`self.HurtBox_BasicAttack`)))) (+ (.yaw (.rotation (`SceneComponent.K2_GetComponentToWorld` (`self.HurtBox_BasicAttack`)))) 0.0))))
          (:`then_1`
            (`/Engine/EditorBlueprintResources/ActorMacros.Switch Has Authority`
              (:`Authority`
                ;[1 1 1] Hit detection
                (`ActorComponent.Activate` _hurtbox_basicattack false)
                (set `PrimitiveComponent.bGenerateOverlapEvents` true _hurtbox_basicattack)
                (`KismetArrayLibrary.Array_Clear` (`self.EnemyHitList`))
                ;[1 1 1] Add owner so they can't be hit by own attacks
                (`KismetArrayLibrary.Array_Add` (`self.EnemyHitList`) (`KismetStringLibrary.Conv_StringToName` (`KismetSystemLibrary.GetObjectName` (`ActorComponent.GetOwner` (`self.HurtBox_BasicAttack`)))))
                ;[1 1 1] Check if we hit a players hit box
                (for _array_element (`PrimitiveComponent.GetOverlappingComponents` (`self.HurtBox_BasicAttack`))
                  (bind (_tagfound _tagname) (`self.CheckAttackTagList` _array_element))
                  (if _tagfound
                    (bind _returnvalue_2 (`ActorComponent.GetOwner` _array_element))
                    ;[1 1 1] Have we hit them before
                    (bind _have_we_hit_them (`self.HaveWeHitBefore` _returnvalue_2 (`self.EnemyHitList`)))
                    (if (not _have_we_hit_them)
                      ;[1 1 1] Deal damage and stagger
                      (switch `name` _tagname
                        (:`PlayerHitBox`
                          (bind _asdefault_player_bp (cast `/Game/Blueprints/PlayerBP/DEFAULT_PLAYER_BP` _returnvalue_2))
                          (`self.StaggerHit` _asdefault_player_bp 10.0 (`SceneComponent.K2_GetComponentLocation` (`self.CapsuleComponent`)) 1.0)
                          (`self.Health_TakeDamage` _asdefault_player_bp 10.0)))))))))))
      (:`PretendAttackEnd`
        (set `self.Attacking` false)
        (`/Engine/EditorBlueprintResources/ActorMacros.Switch Has Authority`
          (:`Authority`
            (`ActorComponent.Deactivate` _hurtbox_basicattack)))))))

(event `self.BasicAttackPressed`
  (`/Engine/EditorBlueprintResources/ActorMacros.Switch Has Authority`
    (:`Authority`
      (`self.Server_BasicAttackPressed`))))

(event `self.BasicAttackActivate`)

(event `self.Server_Ability1Pressed`
  (bind _cat_ability1_phasematerial (`self.Cat_Ability1_PhaseMaterial`))
  (bind _mesh (`self.Mesh`))
  ;[1 1 1] Checks
  (if (and (not (`self.Attacking`)) (not (`self.IsRagdolled`)) (<= (`self.Ability1CoolDown_Timer`) 0.0))
    (`GameplayStatics.PlaySoundAtLocation` "/Game/Sounds/Cat/Cat_TACTICAL_ATTACK_Stereo_48k_24-bit.Cat_TACTICAL_ATTACK_Stereo_48k_24-bit" (0.0 0.0 0.0) (struct) 1.0 1.0 0.0 null null null)
    ;[1 1 1] Disable hitboxes + speed boost
    (`KismetSystemLibrary.Delay` 1.0)
    (`PrimitiveComponent.SetCollisionProfileName` (`self.HitBox`) "NoCollision" true)
    (`PrimitiveComponent.SetCollisionProfileName` (`self.HitBoxArms`) "NoCollision" true)
    (`self.UpdateUnmodifiedMovespeed` 900.0)
    ;[1 1 1] Start timer
    (set `self.Ability1_UseTimer` (`self.Ability1_UseDuration`))
    ;[1 1 1] Visuals
    (`PrimitiveComponent.SetMaterial` _mesh 0 _cat_ability1_phasematerial)
    (`PrimitiveComponent.SetMaterial` _mesh 1 _cat_ability1_phasematerial)
    ;[1 1 1] Event tick toggle
    (set `self.Ability1_Using` true)))

(event `self.Ability1Pressed`
  (`/Engine/EditorBlueprintResources/ActorMacros.Switch Has Authority`
    (:`Authority`
      (`self.Server_Ability1Pressed`))))

(event `self.Ability1Activate`)

(event `self.Server_Ability2Pressed`
  (bind _capsulecomponent (`self.CapsuleComponent`))
  ;[1 1 1] Checks
  (if (and (not (`self.Attacking`)) (not (`self.IsRagdolled`)) (<= (`self.Ability2CoolDown_Timer`) 0.0))
    ;[1 1 1] Buildup
    (set `self.Attacking` true) ; Consume input
    (`self.UpdateUnmodifiedMovespeed` 0.0)
    (`|ExecutionSequence`
      (:`then_0`
        ;[1 1 1] Animations
        (`self.PlayAnimMontage` (`|GetArrayItem` (`self.AnimMontageArray`) 1))
        (bind _ascat_anim_bp (cast `/Game/Anims/Cat/Cat_AnimBP` (`SkeletalMeshComponent.GetAnimInstance` (`self.Mesh`))))
        (set `/Game/Anims/Cat/Cat_AnimBP.FullyBodyAnimOverride` true _ascat_anim_bp)
        (bind (_direction _blendweight) (`Timeline|FakeAnimSummon` :!via `PlayFromStart`)
          (:`Update`
            (`self.PhysicalAnimTrigger` true _blendweight) ; Blend from animation to ragdoll to prevent snapping
          )
          (:`Finished`
            (set `/Game/Anims/Cat/Cat_AnimBP.FullyBodyAnimOverride` false _ascat_anim_bp)
            ;[1 1 1] Spawn
            (`/Engine/EditorBlueprintResources/ActorMacros.Switch Has Authority`
              (:`Authority`
                (`self.SpawnTheFingCerberus`))
              (:`Remote`
                _))
            (`self.UpdateUnmodifiedMovespeed` (`self._DefaultWalkSpeed_`))
            (set `self.Attacking` false) ; Consume input
            ;[0 0.3383 1] COOLDOWN
            (`self.SetAbility2_OnCooldown` 1.0))))
      (:`then_1`
        ;[1 1 1] Particles
        (`GameplayStatics.SpawnEmitterAttached` "/Game/ParticlesBP/Cat/CatSummon.CatSummon" _capsulecomponent "None" (0.0 100.0 -60.0) (struct :`Yaw` -90.0) (0.3 0.3 0.3))
        (`GameplayStatics.SpawnEmitterAttached` "/Game/ParticlesBP/Cat/CatSummon.CatSummon" _capsulecomponent "None" (0.0 -100.0 -60.0) (struct :`Yaw` -90.0) (0.3 0.3 0.3))
        (`GameplayStatics.SpawnEmitterAttached` "/Game/ParticlesBP/Cat/CatSummon.CatSummon" _capsulecomponent "None" (100.0 0.0 -60.0) (struct :`Yaw` -90.0) (0.3 0.3 0.3))))))

(event `self.Ability2Pressed`
  (`/Engine/EditorBlueprintResources/ActorMacros.Switch Has Authority`
    (:`Authority`
      (`self.Server_Ability2Pressed`))))

(event `self.Ability2Activate`)

(event `Ability1End`
  (`/Engine/EditorBlueprintResources/ActorMacros.Switch Has Authority`
    (:`Authority`
      (`self.Server_Ability1End`))))

(event `Server_Ability1End`
  (bind _mesh (`self.Mesh`))
  ;[1 1 1] Reset when time is up
  (set `self.Ability1_Using` false)
  (set `self.Attacking` false)
  (`self.UpdateUnmodifiedMovespeed` (`self._DefaultWalkSpeed_`))
  (`PrimitiveComponent.SetMaterial` _mesh 0 (`self.Cat_DefaultModelMaterial`))
  (`PrimitiveComponent.SetMaterial` _mesh 1 "/Game/Materials/Cat/Cat_BaseColourEye.Cat_BaseColourEye")
  (`self.SetAbility1_OnCooldown` 1.0)
  (`PrimitiveComponent.SetCollisionProfileName` (`self.HitBox`) "OverlapAll" true)
  (`PrimitiveComponent.SetCollisionProfileName` (`self.HitBoxArms`) "OverlapAll" true))

(event `self.ReceiveTick`
  (params (DeltaSeconds :type "Float (single-precision)"))
  (`parent.ReceiveTick` DeltaSeconds)
  (`|ExecutionSequence`
    (:`then_0`
      ;[1 1 1] While ability 1 is active
      (if (`self.Ability1_Using`)
        (set `self.Attacking` true) ; Consume input
        (bind _output_get (set `self.Ability1_UseTimer` (- (`self.Ability1_UseTimer`) (`GameplayStatics.GetWorldDeltaSeconds`))))
        (if (<= _output_get 0.0)
          (`self.Ability1End`))))))

(event `self.ReceiveDestroyed`)

(fn `SpawnTheFingCerberus`
  (bind _capsulecomponent (`self.CapsuleComponent`))
  (bind _capsulecomponent_2 (`self.CapsuleComponent`))
  (bind _capsulecomponent_3 (`self.CapsuleComponent`))
  (`|ExecutionSequence`
    (:`then_0`
      ;[1 1 1] Minion 1
      (bind _returnvalue (`|SpawnActorFromClass` "/Game/AI/CatAI/Cat_UltimateAI_BP.Cat_UltimateAI_BP_C" (`KismetMathLibrary.MakeTransform` (+ (.location (`SceneComponent.K2_GetComponentToWorld` _capsulecomponent)) (* (`SceneComponent.GetForwardVector` _capsulecomponent) 100.0)) (.rotation (`SceneComponent.K2_GetComponentToWorld` _capsulecomponent)) (0.6 0.6 0.6)) "Undefined" "OverrideRootScale" null null))
      (set `/Game/AI/CatAI/Cat_UltimateAI_BP.CatOwnerName` (`KismetStringLibrary.Conv_StringToName` (`KismetSystemLibrary.GetObjectName` self)) _returnvalue))
    (:`then_1`
      ;[1 1 1] Minion 2
      (bind _returnvalue_2 (`|SpawnActorFromClass` "/Game/AI/CatAI/Cat_UltimateAI_BP.Cat_UltimateAI_BP_C" (`KismetMathLibrary.MakeTransform` (+ (.location (`SceneComponent.K2_GetComponentToWorld` _capsulecomponent_2)) (* (`SceneComponent.GetRightVector` _capsulecomponent_2) 100.0)) (.rotation (`SceneComponent.K2_GetComponentToWorld` _capsulecomponent_2)) (0.6 0.6 0.6)) "Undefined" "OverrideRootScale" null null))
      (set `/Game/AI/CatAI/Cat_UltimateAI_BP.CatOwnerName` (`KismetStringLibrary.Conv_StringToName` (`KismetSystemLibrary.GetObjectName` self)) _returnvalue_2))
    (:`then_2`
      ;[1 1 1] Minion 3
      (bind _returnvalue_3 (`|SpawnActorFromClass` "/Game/AI/CatAI/Cat_UltimateAI_BP.Cat_UltimateAI_BP_C" (`KismetMathLibrary.MakeTransform` (+ (.location (`SceneComponent.K2_GetComponentToWorld` _capsulecomponent_3)) (* (`SceneComponent.GetRightVector` _capsulecomponent_3) -100.0)) (.rotation (`SceneComponent.K2_GetComponentToWorld` _capsulecomponent_3)) (0.6 0.6 0.6)) "Undefined" "OverrideRootScale" null null))
      (set `/Game/AI/CatAI/Cat_UltimateAI_BP.CatOwnerName` (`KismetStringLibrary.Conv_StringToName` (`KismetSystemLibrary.GetObjectName` self)) _returnvalue_3))))

(fn `UserConstructionScript`
  (`parent.UserConstructionScript`))