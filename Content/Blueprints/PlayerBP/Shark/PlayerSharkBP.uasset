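; Shark player character with an alternating punch, a wave dash and an ultimate that summons a wave actor.
; Input events run on authority, with timelines timing the punch hurt box and the movement-locked ultimate cast.
; The dash hides the mesh, disables hit boxes and drives velocity from Tick, then restores everything and starts cooldown.
; Punch and dash damage and stagger overlapped players, filtered by tag and an already-hit list.
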(event `self.Server_BasicAttackPressed`
  (bind _hurtbox_basicattack (`self.HurtBox_BasicAttack`))
  (bind _animmontagearray (`self.AnimMontageArray`))
  (bind _hurtbox_basicattack_2 (`self.HurtBox_BasicAttack`))
  ;[1 1 1] Checks
  (if (and (not (`self.Attacking`)) (not (`self.IsRagdolled`)))
    (set `self.Attacking` true)
    ;[1 1 1] Flip flop the punch animations
    (`/Engine/EditorBlueprintResources/StandardMacros.FlipFlop`
      (:`A`
        (`self.PlayAnimMontage` (`|GetArrayItem` _animmontagearray)))
      (:`B`
        (`self.PlayAnimMontage` (`|GetArrayItem` _animmontagearray 1))))
    (`|ExecutionSequence`
      (:`then_0`
        (`Timeline|FakeBasicAttackAnimation` :!via `PlayFromStart`
          (:`Finished`
            (set `self.Attacking` false))
          (:`PretendAttackStart`
            ;[1 1 1] PARTICLE
            (`GameplayStatics.SpawnEmitterAttached` "/Game/ParticlesBP/Sharkgirl/SharkPunchRight.SharkPunchRight" _hurtbox_basicattack_2 "None" (+ (.location (`SceneComponent.GetRelativeTransform` _hurtbox_basicattack_2)) (-50.0 0.0 0.0)) (`KismetMathLibrary.MakeRotator` (.roll (.rotation (`SceneComponent.GetRelativeTransform` _hurtbox_basicattack_2))) (+ (.pitch (.rotation (`SceneComponent.GetRelativeTransform` _hurtbox_basicattack_2))) 180.0) (.yaw (.rotation (`SceneComponent.GetRelativeTransform` _hurtbox_basicattack_2)))) (0.5 0.7 1.0))
            ;[1 1 1] Default activation
            (`ActorComponent.Activate` _hurtbox_basicattack false)
            (`PrimitiveComponent.SetCollisionProfileName` _hurtbox_basicattack "OverlapAll" true)
            (`KismetArrayLibrary.Array_Clear` (`self.EnemyHitList`))
            (`/Engine/EditorBlueprintResources/ActorMacros.Switch Has Authority`
              (:`Authority`
                ;[1 1 1] Add owner so they cant get hit by own attacks
                (`KismetArrayLibrary.Array_Add` (`self.EnemyHitList`) (`KismetStringLibrary.Conv_StringToName` (`KismetSystemLibrary.GetObjectName` (`ActorComponent.GetOwner` (`self.HurtBox_BasicAttack`)))))
                ;[1 1 1] Check if we hit a players hit box
                (for _array_element (`PrimitiveComponent.GetOverlappingComponents` (`self.HurtBox_BasicAttack`))
                  (bind (_tagfound _tagname) (`self.CheckAttackTagList` _array_element))
                  (if _tagfound
                    (bind _returnvalue (`ActorComponent.GetOwner` _array_element))
                    ;[1 1 1] Have we hit them before
                    (bind _have_we_hit_them (`self.HaveWeHitBefore` _returnvalue (`self.EnemyHitList`)))
                    (if (not _have_we_hit_them)
                      ;[1 1 1] Deal damage and stagger
                      (switch `name` _tagname
                        (:`PlayerHitBox`
                          (bind _asdefault_player_bp (cast `/Game/BluePrints/PlayerBP/DEFAULT_PLAYER_BP` _returnvalue))
                          (`self.StaggerHit` _asdefault_player_bp 10.0 (`SceneComponent.K2_GetComponentLocation` (`self.CapsuleComponent`)) 1.0)
                          (`self.Health_TakeDamage` _asdefault_player_bp 10.0)))))))))
          (:`PretendAttackEnd`
            (`ActorComponent.Deactivate` _hurtbox_basicattack)
            (`PrimitiveComponent.SetCollisionProfileName` _hurtbox_basicattack "NoCollision" true)))))))

(event `self.BasicAttackPressed`
  (`/Engine/EditorBlueprintResources/ActorMacros.Switch Has Authority`
    (:`Authority`
      (`self.Server_BasicAttackPressed`))))

(event `self.BasicAttackActivate`)

(event `self.ReceiveBeginPlay`
  (`parent.ReceiveBeginPlay`)
  ;[1 1 1] Cooldowns
  (set `self._Ability1CoolDown_Duration` (`self.Shark_Ability1_CooldownDuration`))
  (set `self._Ability2CoolDown_Duration` (`self.Shark_Ability2_CooldownDuration`))
  ;[1 1 1] Bone Setting
  (set `self.ShieldBoneAttachPoint` "bn_pelvis01")
  (set `self.ShieldSize` (0.05 0.05 0.05))
  (set `self.PhysicsStartPoint` "bn_torso01")
  (`self.PhysicalAnimTrigger` true))

(event `self.Server_Ability1Pressed`
  (bind _returnvalue (`SceneComponent.K2_GetComponentRotation` (`self.CapsuleComponent`)))
  ;[1 1 1] Checks
  (if (and (not (`self.Attacking`)) (not (`self.IsRagdolled`)) (<= (`self.Ability1CoolDown_Timer`) 0.0))
    ;[1 1 1] Visibility and collider toggle
    (`PrimitiveComponent.SetCollisionProfileName` (`self.HitBox`) "NoCollision" true)
    (`PrimitiveComponent.SetCollisionProfileName` (`self.HitBoxArms`) "NoCollision" true)
    (`PrimitiveComponent.SetCollisionProfileName` (`self.Ability1HurtBox`) "OverlapAll" true)
    (`SceneComponent.SetVisibility` (`self.Mesh`) false false)
    (`SceneComponent.SetVisibility` (`self.WaveDash`) true false)
    (`SceneComponent.SetVisibility` (`self.WaveDashWasher2`) true false)
    (`ActorComponent.Activate` (`self.WaveDashParticle`) false)
    (`GameplayStatics.PlaySoundAtLocation` "/Game/Sounds/Shark/Shark_TACTICAL_ATTACK_Stereo_48k_24-bit.Shark_TACTICAL_ATTACK_Stereo_48k_24-bit" (0.0 0.0 0.0) (struct) 1.0 1.0 0.0 null null null)
    ;[1 1 1] Activate Dash
    (set `CharacterMovementComponent.RotationRate` (struct) (`self.CharacterMovement`))
    (set `self.SharkDashForwardRotation` _returnvalue)
    (set `self.SharkDashForwardDirection` (`KismetMathLibrary.GetForwardVector` _returnvalue))
    (set `self.SharkDashTimer` (`self._SharkDashDuration`))
    (set `self.SharkDashOn` true)
    ;[1 1 1] Normal Hit detection stuff
    (`KismetArrayLibrary.Array_Clear` (`self.EnemyHitList`))
    (`KismetArrayLibrary.Array_Add` (`self.EnemyHitList`) (`KismetStringLibrary.Conv_StringToName` (`KismetSystemLibrary.GetObjectName` (`ActorComponent.GetOwner` (`self.HurtBox_BasicAttack`)))))))

(event `self.Ability1Pressed`
  (`/Engine/EditorBlueprintResources/ActorMacros.Switch Has Authority`
    (:`Authority`
      (`self.Server_Ability1Pressed`))))

(event `self.Ability1Activate`)

(event `self.Server_Ability2Pressed`
  (bind _ultimatespawnpoint (`self.UltimateSpawnPoint`))
  ;[1 1 1] Checks
  (if (and (not (`self.Attacking`)) (not (`self.IsRagdolled`)) (<= (`self.Ability2CoolDown_Timer`) 0.0))
    (set `self.Attacking` true)
    ;[1 1 1] Animation
    (`GameplayStatics.PlaySoundAtLocation` "/Game/Sounds/Shark/Shark_ULTIMATE_ATACK_Stereo_48k_24-bit.Shark_ULTIMATE_ATACK_Stereo_48k_24-bit" (0.0 0.0 0.0) (struct) 1.0 1.0 0.0 null null null)
    (bind _assharkgirl_anim_bp (cast `/Game/Anims/Sharkgirl/Sharkgirl_AnimBP` (`SkeletalMeshComponent.GetAnimInstance` (`self.Mesh`))))
    (set `/Game/Anims/Sharkgirl/Sharkgirl_AnimBP.FullbodyAnimOverride` true _assharkgirl_anim_bp)
    (`self.PlayAnimMontage` (`|GetArrayItem` (`self.AnimMontageArray`) 4))
    (`GameplayStatics.SpawnEmitterAttached` "/Game/ParticlesBP/Sharkgirl/WaveSummonShark.WaveSummonShark" (`self.Mesh`) "None" (0.0 0.0 0.0) (struct) (0.65 0.65 0.65))
    (`GameplayStatics.SpawnEmitterAttached` "/Game/ParticlesBP/Sharkgirl/SharkgirlWaveCreate_Begin.SharkgirlWaveCreate_Begin" _ultimatespawnpoint "None" (+ (.location (`SceneComponent.GetRelativeTransform` _ultimatespawnpoint)) (-200.0 0.0 0.0)) (`KismetMathLibrary.MakeRotator` (.roll (.rotation (`SceneComponent.GetRelativeTransform` _ultimatespawnpoint))) (.pitch (.rotation (`SceneComponent.GetRelativeTransform` _ultimatespawnpoint))) (+ (.yaw (.rotation (`SceneComponent.GetRelativeTransform` _ultimatespawnpoint))) 90.0)) (0.4 0.4 0.4))
    (`Timeline|FakeUltimateAnimation` :!via `PlayFromStart`
      (:`Finished`
        ;[1 1 1] Reset movement stuff
        (`self.UpdateUnmodifiedMovespeed` (`self._DefaultWalkSpeed_`))
        (set `CharacterMovementComponent.RotationRate` (`self._DefaultRotationRate_`) (`self.CharacterMovement`))
        (set `self.Attacking` false)
        (`self.SetAbility2_OnCooldown` 1.0)
        (`GameplayStatics.SpawnEmitterAtLocation` "/Game/ParticlesBP/Sharkgirl/SharkgirlWaveCreate_End.SharkgirlWaveCreate_End" (+ (.location (`SceneComponent.K2_GetComponentToWorld` (`self.UltimateSpawnPoint`))) (0.0 0.0 0.0)) (`KismetMathLibrary.MakeRotator` (.roll (.rotation (`SceneComponent.K2_GetComponentToWorld` (`self.UltimateSpawnPoint`)))) (.pitch (.rotation (`SceneComponent.K2_GetComponentToWorld` (`self.UltimateSpawnPoint`)))) (+ (.yaw (.rotation (`SceneComponent.K2_GetComponentToWorld` (`self.UltimateSpawnPoint`)))) 90.0)) (0.4 0.4 0.4)))
      (:`StartAnim`
        ;[1 1 1] Ultimate movement lockouts
        (`self.UpdateUnmodifiedMovespeed` 0.0)
        (set `CharacterMovementComponent.RotationRate` (struct) (`self.CharacterMovement`)))
      (:`UltimateCast`
        ;[1 1 1] Spawn wave object
        (`/Engine/EditorBlueprintResources/ActorMacros.Switch Has Authority`
          (:`Authority`
            (bind _returnvalue (`|SpawnActorFromClass` "/Game/BluePrints/PlayerBP/Shark/PlayerShark_UltimateSpawnable.PlayerShark_UltimateSpawnable_C" (`SceneComponent.K2_GetComponentToWorld` (`self.UltimateSpawnPoint`)) "Undefined" "OverrideRootScale" null null))
            (set `/Game/BluePrints/PlayerBP/Shark/PlayerShark_UltimateSpawnable.OwningPlayer` self _returnvalue)
            (set `/Game/Anims/Sharkgirl/Sharkgirl_AnimBP.FullbodyAnimOverride` false _assharkgirl_anim_bp)))))))

(event `self.Ability2Pressed`
  (`/Engine/EditorBlueprintResources/ActorMacros.Switch Has Authority`
    (:`Authority`
      (`self.Server_Ability2Pressed`))))

(event `self.Ability2Activate`)

(event `SharkDash`
  (`/Engine/EditorBlueprintResources/ActorMacros.Switch Has Authority`
    (:`Authority`
      (`self.Server_SharkDash`))))

(event `Server_SharkDash`)

(event `self.ReceiveTick`
  (params (DeltaSeconds :type "Float (single-precision)"))
  (bind _charactermovement (`self.CharacterMovement`))
  (`parent.ReceiveTick` DeltaSeconds)
  (`|ExecutionSequence`
    (:`then_0`
      (if (`self.SharkDashOn`)
        ;[1 1 1] Check if we've run out of time
        (bind _output_get (set `self.SharkDashTimer` (- (`self.SharkDashTimer`) (`GameplayStatics.GetWorldDeltaSeconds`))))
        (if (> _output_get 0.0)
          ;[1 1 1] Dashing movement + consume
          (`/Engine/EditorBlueprintResources/ActorMacros.Switch Has Authority`
            (:`Authority`
              (set `CharacterMovementComponent.MaxWalkSpeed` 1500.0 _charactermovement) ; Bypass speed mods
              (set `MovementComponent.Velocity` (* (`self.SharkDashForwardDirection`) 2000.0) _charactermovement)
              (`SceneComponent.K2_SetWorldRotation` (`self.Ability1HurtBox`) (`self.SharkDashForwardRotation`) false false)
              (set `self.Attacking` true)
              (`/Engine/EditorBlueprintResources/ActorMacros.Switch Has Authority`
                (:`Authority`
                  ;[1 1 1] Check if we hit a players hit box
                  (for _array_element (`PrimitiveComponent.GetOverlappingComponents` (`self.Ability1HurtBox`))
                    (bind (_tagfound _tagname) (`self.CheckAttackTagList` _array_element))
                    (if _tagfound
                      (bind _returnvalue (`ActorComponent.GetOwner` _array_element))
                      ;[1 1 1] Have we hit them before
                      (bind _have_we_hit_them (`self.HaveWeHitBefore` _returnvalue (`self.EnemyHitList`)))
                      (if (not _have_we_hit_them)
                        ;[1 1 1] Deal damage and stagger
                        (switch `name` _tagname
                          (:`PlayerHitBox`
                            (bind _asdefault_player_bp (cast `/Game/BluePrints/PlayerBP/DEFAULT_PLAYER_BP` _returnvalue))
                            (`self.StaggerHit` _asdefault_player_bp 10.0 (`SceneComponent.K2_GetComponentLocation` (`self.CapsuleComponent`)) 1.0)
                            (`self.Health_TakeDamage` _asdefault_player_bp 10.0))))))))))
          (else
            ;[1 1 1] Reset everything
            (`self.UpdateUnmodifiedMovespeed` (`self._DefaultWalkSpeed_`))
            (set `CharacterMovementComponent.RotationRate` (`self._DefaultRotationRate_`) (`self.CharacterMovement`))
            (set `self.SharkDashOn` false)
            (set `self.Attacking` false)
            (`self.SetAbility1_OnCooldown` 1.0)
            (`PrimitiveComponent.SetCollisionProfileName` (`self.HitBox`) "OverlapAll" true)
            (`PrimitiveComponent.SetCollisionProfileName` (`self.HitBoxArms`) "OverlapAll" true)
            (`PrimitiveComponent.SetCollisionProfileName` (`self.Ability1HurtBox`) "NoCollision" true)
            (`SceneComponent.SetVisibility` (`self.Mesh`) true false)
            (`SceneComponent.SetVisibility` (`self.WaveDash`) false false)
            (`SceneComponent.SetVisibility` (`self.WaveDashWasher2`) false false)
            (`ActorComponent.Deactivate` (`self.WaveDashParticle`))
            (set `MovementComponent.Velocity` (* (`self.SharkDashForwardDirection`) 400.0) (`self.CharacterMovement`))
            ;[1 1 1] Animation
            (bind _assharkgirl_anim_bp (cast `/Game/Anims/Sharkgirl/Sharkgirl_AnimBP` (`SkeletalMeshComponent.GetAnimInstance` (`self.Mesh`))))
            (set `/Game/Anims/Sharkgirl/Sharkgirl_AnimBP.FullbodyAnimOverride` true _assharkgirl_anim_bp)
            (bind _returnvalue_2 (`self.PlayAnimMontage` (`|GetArrayItem` (`self.AnimMontageArray`) 3)))
            (`KismetSystemLibrary.Delay` _returnvalue_2)
            (set `/Game/Anims/Sharkgirl/Sharkgirl_AnimBP.FullbodyAnimOverride` false _assharkgirl_anim_bp)))))))

(fn `UserConstructionScript`
  (`parent.UserConstructionScript`))