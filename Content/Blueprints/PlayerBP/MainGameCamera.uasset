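; Shared multiplayer camera that frames every actor tagged "Player" with a single spring-arm view.
; Each tick it eases its root toward the players' average location and sets arm length from the furthest player's distance, with a minimum zoom threshold.
; Rotation blends smoothly toward a target that outside Blueprints set through ChangeRotation.
; With no players present, it drifts back to a waiting point.
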(event `self.ReceiveBeginPlay`
  (bind _defaultrotation (`self.DefaultRotation`))
  ;[1 1 1] Get all players
  (bind _outactors (`GameplayStatics.GetAllActorsWithTag` "Player"))
  (set `self.ListOfPlayers` _outactors)
  ;[1 1 1] Rotation stuff
  (set `self.NewRotation` _defaultrotation)
  (set `self.CurrentRotation` _defaultrotation))

(event `self.ReceiveTick`
  (params (DeltaSeconds :type "Float (single-precision)"))
  (bind _root (`self.Root`))
  (bind _distancechangethreshold (`self.DistanceChangeThreshold`))
  (bind _furthestdistance (`self.FurthestDistance`))
  (bind _springarm (`self.SpringArm`))
  (bind _camerazoommultipler (`self.CameraZoomMultipler`))
  (bind _listofplayers (`self.ListOfPlayers`))
  (bind _returnvalue (`KismetMathLibrary.RInterpTo` (`self.CurrentRotation`) (`self.NewRotation`) DeltaSeconds 1.0))
  (bind _targetarmlength (`SpringArmComponent.TargetArmLength` (`self.SpringArm`)))
  ;[1 1 1] Get all players
  (bind _outactors (`GameplayStatics.GetAllActorsWithTag` "Player"))
  (bind _output_get (set `self.ListOfPlayers` _outactors))
  (if (`KismetArrayLibrary.Array_IsValidIndex` _output_get)
    ;[1 1 1] Move to the average location of all players
    (bind _returnvalue_2 (`GameplayStatics.GetActorArrayAverageLocation` _listofplayers))
    (if (not (<= (`KismetArrayLibrary.Array_Length` _listofplayers) 0))
      (`SceneComponent.K2_SetWorldLocation` (`self.Root`) (`KismetMathLibrary.VInterpTo` (`SceneComponent.K2_GetComponentLocation` (`self.Root`)) _returnvalue_2 DeltaSeconds 2.0) false true)
      ;[1 1 1] Calculate the distance between the camera point and the furthest player
      (set `self.FurthestDistance` 0.0)
      (for _array_element (`self.ListOfPlayers`)
        (bind _returnvalue_3 (`KismetMathLibrary.Vector_Distance` (`SceneComponent.K2_GetComponentLocation` (`self.Root`)) (`self.K2_GetActorLocation` _array_element)))
        (if (> _returnvalue_3 (`self.FurthestDistance`))
          (set `self.FurthestDistance` _returnvalue_3)))
      ;[1 1 1] Adjust camera length based on player distance apart
      (if (> _furthestdistance _distancechangethreshold)
        (set `SpringArmComponent.TargetArmLength` (`KismetMathLibrary.FInterpTo` _targetarmlength (* _furthestdistance _camerazoommultipler) DeltaSeconds 1.0) _springarm)
        (else
          (set `SpringArmComponent.TargetArmLength` (`KismetMathLibrary.FInterpTo` _targetarmlength (* _distancechangethreshold _camerazoommultipler) DeltaSeconds 1.0) _springarm)))
      ;[1 1 1] Interpolate between rotations
      (`SceneComponent.K2_SetWorldRotation` (`self.SpringArm`) _returnvalue false false)
      (set `self.CurrentRotation` _returnvalue))
    (else
      ;[1 1 1] reset back to waiting point when no players exist
      (`SceneComponent.K2_SetWorldLocation` _root (`KismetMathLibrary.VInterpTo` (`SceneComponent.K2_GetComponentLocation` _root) (`self.WaitingPoint`) DeltaSeconds 1.0) false true))))

(event `ChangeRotation`
  (params (NewRotation :type "Rotator Structure"))
  ;[1 1 1] Change rotation function to access from outside
  (set `self.NewRotation` NewRotation))

(fn `UserConstructionScript`)