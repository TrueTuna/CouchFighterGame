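; Playable Teddy bear character with a melee punch and two cooldown abilities, built on shared parent player logic.
; Attack inputs play montages gated by ragdoll and Attacking state, with physical animation toggled around the punch.
; Punch and ultimate damage and stagger tagged hurtbox overlaps once per target, while Ability 1 spawns a jaws attack actor.
; The ultimate roots Teddy in a summoning circle before a delayed heavy hit, with Tick holding Attacking throughout.
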(event `self.BasicAttackPressed`
  ;[1 1 1] Playing punch animation
  (if (and (not (`self.IsRagdolled`)) (not (`self.Attacking`)))
    (set `self.Attacking` true)
    (`self.PhysicalAnimTrigger` false)
    (bind _returnvalue (`self.PlayAnimMontage` (`|GetArrayItem` (`self.AnimMontageArray`))))
    (`KismetSystemLibrary.Delay` (/ _returnvalue 1.2))
    (`self.PhysicalAnimTrigger` true)
    (set `self.Attacking` false)))

(event `self.ReceiveBeginPlay`
  ;[1 1 1] BEGIN
  (`parent.ReceiveBeginPlay`)
  (set `self.PlayerShieldFX` "/Game/ParticlesBP/Robot/Robot_Shield.Robot_Shield")
  (set `self._Ability1CoolDown_Duration` (`self.Teddy_Ability1Cooldown_Duration`))
  (set `self._Ability2CoolDown_Duration` (`self.Teddy_Ability2Cooldown_Duration`)))

(event `BasicAttackCharge`
  ;[1 1 1] Spawn attack particle 1
  (`GameplayStatics.SpawnEmitterAttached` "/Game/ParticlesBP/Teddy/BasicAttack_BodySlash.BasicAttack_BodySlash" (`self.HurtBox_BasicAttack`) "None" (-50.0 0.0 0.0) (struct) (1.0 0.25 1.0)))

(event `BasicAttackActivate`
  (bind _hurtbox_basicattack (`self.HurtBox_BasicAttack`))
  ;[1 1 1] Basic attacks Start
  (`ActorComponent.Activate` _hurtbox_basicattack false)
  (set `PrimitiveComponent.bGenerateOverlapEvents` true _hurtbox_basicattack)
  (`KismetArrayLibrary.Array_Clear` (`self.EnemyHitList`))
  ;[1 1 1] Add owner to the list so they can't get hit by their own attack
  (`KismetArrayLibrary.Array_Add` (`self.EnemyHitList`) (`KismetStringLibrary.Conv_StringToName` (`KismetSystemLibrary.GetObjectName` (`ActorComponent.GetOwner` (`self.HurtBox_BasicAttack`)))))
  ;[1 1 1] Check if the attack box hits a player's hitbox
  (for _array_element (`PrimitiveComponent.GetOverlappingComponents` (`self.HurtBox_BasicAttack`))
    (bind (_tagfound _tagname) (`self.CheckAttackTagList` _array_element))
    (if _tagfound
      (bind _returnvalue (`ActorComponent.GetOwner` _array_element))
      ;[1 1 1] Have we hit them before
      (bind _have_we_hit_them (`self.HaveWeHitBefore` _returnvalue (`self.EnemyHitList`)))
      (if (not _have_we_hit_them)
        ;[1 1 1] Deal damage and stagger
        (switch `name` _tagname
          (:`PlayerHitBox`
            (bind _asdefault_player_bp (cast `/Game/Blueprints/PlayerBP/DEFAULT_PLAYER_BP` _returnvalue))
            (`self.StaggerHit` _asdefault_player_bp 10.0 (`SceneComponent.K2_GetComponentLocation` (`self.CapsuleComponent`)) 1.0)
            (`self.Health_TakeDamage` _asdefault_player_bp 10.0)))))))

(event `BasicAttackDeactivate`
  ;[1 1 1] Basic attacks Start
  (`ActorComponent.Deactivate` (`self.HurtBox_BasicAttack`)))

(event `self.ReceiveTick`
  (params (DeltaSeconds :type "Float (single-precision)"))
  ;[1 1 1] Event Tick
  (`parent.ReceiveTick` DeltaSeconds)
  (`|ExecutionSequence`
    (:`then_0`
      ;[1 0.4993 0] Keep attacking on to prevent other attacks midway through ultimate / MAKE BETTER
      (if (`self.UltimateOn`)
        (set `self.Attacking` true)
        (goto _label :!via `Reset`)
        (else
          (`/Engine/EditorBlueprintResources/StandardMacros.DoOnce` false :!label _label
            (:`Completed`
              (set `self.Attacking` false))))))))

(event `self.Ability1Pressed`
  ;[1 1 1] Playing ability 1 anim
  (if (and (not (`self.IsRagdolled`)) (not (`self.Attacking`)) (<= (`self.Ability1CoolDown_Timer`) 0.0))
    (set `self.Attacking` true)
    (`self.SetAbility1_OnCooldown` 1.0)
    (`self.PhysicalAnimTrigger` true)
    (bind _returnvalue (`self.PlayAnimMontage` (`|GetArrayItem` (`self.AnimMontageArray`) 1)))
    (`KismetSystemLibrary.Delay` (/ _returnvalue 1.0))
    (`self.PhysicalAnimTrigger` true)
    (set `self.Attacking` false)))

(event `Ability1Activate`
  (bind _hurtbox_ability1 (`self.HurtBox_Ability1`))
  ;[1 1 1] Ability 1 Start
  (`ActorComponent.Activate` _hurtbox_ability1 false)
  (set `PrimitiveComponent.bGenerateOverlapEvents` true _hurtbox_ability1)
  (`KismetArrayLibrary.Array_Clear` (`self.EnemyHitList`))
  ;[1 1 1] Spawning jaws
  (bind _returnvalue (`|SpawnActorFromClass` :`Class` "/Game/Blueprints/PlayerBP/Teddy/Teddy_Ability1_Spawnable.Teddy_Ability1_Spawnable_C" :`SpawnTransform` (`KismetMathLibrary.MakeTransform` (.location (`SceneComponent.K2_GetComponentToWorld` (`self.HurtBox_Ability1`))) (.rotation (`SceneComponent.K2_GetComponentToWorld` (`self.HurtBox_Ability1`)))) :`CollisionHandlingOverride` "Undefined" :`TransformScaleMethod` "OverrideRootScale" :`OwningPlayer` null :`Instigator` null))
  ;[1 1 1] Actor fucntion
  (set `/Game/Blueprints/PlayerBP/Teddy/Teddy_Ability1_Spawnable.OwningPlayer` self _returnvalue)
  (set `/Game/Blueprints/PlayerBP/Teddy/Teddy_Ability1_Spawnable.TagsToLookFor` (`self.AttackTagToLookFor`) _returnvalue)
  (`/Game/Blueprints/PlayerBP/Teddy/Teddy_Ability1_Spawnable.JawsAttack` _returnvalue))

(event `self.ReceiveDestroyed`
  (bind _defconlaserref (`self.DefconLaserRef`))
  (bind _lasereyeoutput (`self.LaserEyeOutput`))
  ;[1 1 1] Upon being destroyed
  (`/Engine/EditorBlueprintResources/StandardMacros.DoOnce` false ; Because Im calling on destrory, it will destroy for multiple frames causing errors
    (:`Completed`
      (if (`KismetSystemLibrary.IsValid` _defconlaserref)
        (`ActorComponent.K2_DestroyComponent` _defconlaserref)
        (if (`KismetSystemLibrary.IsValid` _lasereyeoutput)
          (`ActorComponent.K2_DestroyComponent` _lasereyeoutput))))))

(event `Ability1Deactivate`
  ;[1 1 1] Ability 1 Start
  (`ActorComponent.Deactivate` (`self.HurtBox_Ability1`)))

(event `self.Ability2Pressed`
  (bind _hurtbox_ability2 (`self.HurtBox_Ability2`))
  (bind _hurtbox_ability2_2 (`self.HurtBox_Ability2`))
  ;[1 1 1] Ultimate ability input
  (if (and (not (`self.IsRagdolled`)) (not (`self.Attacking`)) (<= (`self.Ability2CoolDown_Timer`) 0.0))
    (set `self.Attacking` true)
    (set `self.UltimateOn` true)
    (`KismetArrayLibrary.Array_Clear` (`self.EnemyHitList`))
    (set `CharacterMovementComponent.MaxWalkSpeed` 0.0 (`self.CharacterMovement`))
    ;[1 1 1] Animation
    (bind _asteddy_anim_bp (cast `/Game/Anims/Teddy/Teddy_AnimBP` (`SkeletalMeshComponent.GetAnimInstance` (`self.Mesh`))))
    (set `/Game/Anims/Teddy/Teddy_AnimBP.FullbodyAnimOverride` true _asteddy_anim_bp)
    (`self.PlayAnimMontage` (`|GetArrayItem` (`self.AnimMontageArray`) 2))
    ;[1 1 1] Ultimate ability damage
    (`GameplayStatics.SpawnEmitterAttached` "/Game/ParticlesBP/Teddy/Teddy_SummoningCircle_Start.Teddy_SummoningCircle_Start" (`self.Mesh`) "ROOT" (0.0 -10.0 0.0) (struct :`Roll` -90.0) (0.65 0.65 0.65))
    (`KismetSystemLibrary.Delay` 2.0)
    (`ActorComponent.Activate` _hurtbox_ability2_2 false)
    (set `PrimitiveComponent.bGenerateOverlapEvents` true _hurtbox_ability2_2)
    ;[1 1 1] Add owner to the list so they can't get hit by their own attack
    (`KismetArrayLibrary.Array_Add` (`self.EnemyHitList`) (`KismetStringLibrary.Conv_StringToName` (`KismetSystemLibrary.GetObjectName` (`ActorComponent.GetOwner` (`self.HurtBox_Ability2`)))))
    ;[1 1 1] Check if the attack box hits a player's hitbox
    (for _array_element (`PrimitiveComponent.GetOverlappingComponents` (`self.HurtBox_Ability2`))
      (bind (_tagfound _tagname) (`self.CheckAttackTagList` _array_element))
      (if _tagfound
        (bind _returnvalue (`ActorComponent.GetOwner` _array_element))
        ;[1 1 1] Have we hit them before
        (bind _have_we_hit_them (`self.HaveWeHitBefore` _returnvalue (`self.EnemyHitList`)))
        (if (not _have_we_hit_them)
          ;[1 1 1] Deal damage and stagger
          (switch `name` _tagname
            (:`PlayerHitBox`
              (bind _asdefault_player_bp (cast `/Game/Blueprints/PlayerBP/DEFAULT_PLAYER_BP` _returnvalue))
              (`self.StaggerHit` _asdefault_player_bp 100.0 (+ (`SceneComponent.K2_GetComponentLocation` _array_element) (0.0 0.0 -100.0)) 10.0)
              (`self.Health_TakeDamage` _asdefault_player_bp 75.0))))))
    (`KismetSystemLibrary.Delay` 0.0)
    ;[1 1 1] Leave ring behind
    (`GameplayStatics.SpawnEmitterAtLocation` "/Game/ParticlesBP/Teddy/Teddy_SummoningCircle_End.Teddy_SummoningCircle_End" (.location (`SceneComponent.GetSocketTransform` (`self.Mesh`) "None" "RTS_World")) (.rotation (`SceneComponent.GetSocketTransform` (`self.Mesh`) "None" "RTS_World")) (0.2 0.2 0.2))
    ;[1 1 1] Ultimate end
    (set `PrimitiveComponent.bGenerateOverlapEvents` true _hurtbox_ability2)
    (`ActorComponent.Deactivate` _hurtbox_ability2)
    (set `CharacterMovementComponent.MaxWalkSpeed` (`self.Teddy_DefaultWalkSpeed`) (`self.CharacterMovement`))
    (set `self.Attacking` false)
    (set `self.UltimateOn` false)
    (bind _asteddy_anim_bp_2 (cast `/Game/Anims/Teddy/Teddy_AnimBP` (`SkeletalMeshComponent.GetAnimInstance` (`self.Mesh`))))
    (set `/Game/Anims/Teddy/Teddy_AnimBP.FullbodyAnimOverride` false _asteddy_anim_bp_2)
    (`self.SetAbility2_OnCooldown` 1.0)))

(fn `UserConstructionScript`
  (`parent.UserConstructionScript`))